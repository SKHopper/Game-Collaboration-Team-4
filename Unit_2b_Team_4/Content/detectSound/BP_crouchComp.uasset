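; BP_crouchComp is a crouch component that slows the player character while crouching.
; On BeginPlay it caches the MaxWalkSpeed of player 0's character movement.
; StartCrouching and StopCrouching events toggle an IsCrouching flag and either scale the cached speed by CrouchSpeedMult or restore it.
; It changes only speed and state, without calling Crouch or resizing the capsule, and always targets player 0 rather than its owner.
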(event EventStopCrouching
  (Variables|Default|SetisCrouching false)
  (Variables|/Script/Engine.CharacterMovementComponent|SetMaxWalkSpeed (Variables|/Script/Engine.Character|GetCharacterMovement (Game|GetPlayerCharacter 0)) (Variables|Default|GetwalkSpeed)))

(event EventStartCrouching
  (Variables|Default|SetisCrouching true)
  (Variables|/Script/Engine.CharacterMovementComponent|SetMaxWalkSpeed (Variables|/Script/Engine.Character|GetCharacterMovement (Game|GetPlayerCharacter 0)) (* (Variables|Default|GetwalkSpeed) (Variables|Default|GetcrouchSpeedMult))))

(event EventBeginPlay
  (Variables|Default|SetwalkSpeed (Variables|/Script/Engine.CharacterMovementComponent|GetMaxWalkSpeed (Variables|/Script/Engine.Character|GetCharacterMovement (Game|GetPlayerCharacter 0)))))