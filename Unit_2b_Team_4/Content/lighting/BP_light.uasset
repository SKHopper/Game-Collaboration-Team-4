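; BP_light is a light actor that brightens as the player pawn gets closer and fades out with distance.
; On BeginPlay it applies its Colour variable to the PointLight component.
; Each Tick it scales Intensity by a clamped linear falloff of the player's distance over Radius and sets that as the light's intensity.
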(event EventTick
  (params (DeltaSeconds :type Float%20%28single-precision%29))
  (Rendering|Components|Light|SetIntensity (Variables|Default|GetPointLight) (* (Variables|Default|Getintensity) (Math|Float|Clamp(Float) (- 1.0 (/ (Transformation|GetDistanceTo (Game|Player|GetPlayerPawn 0) self) (Variables|Default|Getradius)))))))

(event EventBeginPlay
  (Rendering|Components|Light|SetLightColor (Variables|Default|GetPointLight) (Variables|Default|Getcolour) true))

(fn ConstructionScript)