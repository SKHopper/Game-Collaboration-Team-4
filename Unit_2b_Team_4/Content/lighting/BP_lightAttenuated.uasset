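; BP_lightAttenuated is a point light actor that fades and hides itself as the player's camera moves away.
; The construction script creates the light component and scales its attenuation radius by a multiplier, and BeginPlay applies the colour and fetches the camera from the player pawn.
; Tick sets intensity by linear distance falloff over Radius, hiding the light at low intensity.
; A randomly seeded toggle runs this update every other frame, staggering instances.
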(event EventTick
  (params (DeltaSeconds :type Float%20%28single-precision%29))
  (bind _self self)
  (bind _radius (Variables|Default|Getradius))
  (bind _camera (Variables|Default|Getcamera))
  (bind _intensity (Variables|Default|Getintensity))
  (bind _returnvalue (Transformation|GetActorLocation _self))
  (bind _returnvalue_2 (Transformation|GetWorldLocation _camera))
  (bind _returnvalue_3 (Math|Vector|Distance(Vector) _returnvalue_2 _returnvalue))
  (bind _returnvalue_4 (/ _returnvalue_3 _radius))
  (bind _returnvalue_5 (- 1.0 _returnvalue_4))
  (bind _returnvalue_6 (Math|Float|Clamp(Float) _returnvalue_5))
  (bind _returnvalue_7 (* _intensity _returnvalue_6 1.0))
  (bind _output_get (Variables|Default|SetNewVar (not (stale _output_get))))
  (if _output_get
    (Rendering|Components|Light|SetIntensity (Variables|Default|Getlight) _returnvalue_7)
    (Rendering|SetVisibility (Variables|Default|Getlight) (> _returnvalue_7 1e+01) false)))

(event EventBeginPlay
  (Rendering|Components|Light|SetLightColor (Variables|Default|Getlight) (Variables|Default|Getcolour) true)
  (bind _camera (Class|IFLight|GetCamforLight(Message) (Game|Player|GetPlayerPawn 0)))
  (Variables|Default|Setcamera _camera)
  (Variables|Default|SetNewVar (Math|Random|RandomBool)))

(fn ConstructionScript
  (bind _light (Variables|Default|Getlight))
  (CallFunction|SetLight)
  (Rendering|Lighting|SetAttenuationRadius _light (* (Variables|/Script/Engine.LocalLightComponent|GetAttenuationRadius _light) (Variables|Default|GetattenMult))))

(fn SetLight
  (bind _returnvalue (AddComponent|AddPointLightComponent false))
  (Variables|Default|Setlight _returnvalue))