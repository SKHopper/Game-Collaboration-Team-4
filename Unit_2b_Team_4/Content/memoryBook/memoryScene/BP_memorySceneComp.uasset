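; Component that plays memory cutscenes, image slides with dialogue, for the intro, book pickups and the ending.
; Scene rows from a data table are picked by memories seen plus books held, then stepped line by line through a widget on each prompt.
; Pickup scenes park the player elsewhere and restore the transform afterwards.
; The intro leads into a level sequence, and the fifth memory triggers the ending and main menu.
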(event Custom|unhideHud
  (Utilities|FlowControl|Delay 3.0)
  (bind _indicator (Default|GetBooksIndicator (Variables|Default|Getplayer)))
  (UserInterface|Viewport|AddtoViewport (Variables|/Game/hud/BP_hudComp.BP_hudComp_C|Gethud (Variables|Default|Gethud)) 0))

(event Custom|fadeInScene
  (bind _widget (Variables|Default|Getwidget))
  (bind _widget_2 (Variables|Default|Getwidget))
  (bind _fadein (Variables|/Game/memoryBook/memoryScene/WBP_memoryScene.WBP_memoryScene_C|GetfadeIn _widget_2))
  (UserInterface|Animation|PlayAnimation _widget_2 _fadein 0.0 1 "Forward" 1.0 false)
  (UserInterface|Viewport|AddtoViewport _widget 0)
  (Default|ResetScene _widget)
  (Utilities|FlowControl|Delay (Class|WidgetAnimation|GetEndTime _fadein))
  (CallFunction|CycleScene))

(event EventPromptNext
  (CallFunction|CycleScene))

(event EventBookPickedUp
  (CallFunction|PlayScene))

(event EventUpdateMemoriesSeen
  (params (returnValue :type Integer))
  (bind _output_get (Variables|Default|SetmemoriesSeen returnValue))
  (if (== _output_get 5)
    (CallFunction|End)))

(event EventBeginPlay
  (bind _returnvalue (UserInterface|CreateWidget "/Game/memoryBook/memoryScene/WBP_memoryScene.WBP_memoryScene_C"))
  (Variables|Default|Setwidget _returnvalue))

(fn PlayScene
  (bind _returnvalue (Game|GetPlayerCharacter 0))
  (bind _memoriesseen (Variables|Default|GetmemoriesSeen))
  (bind _scenesdata (Variables|Default|GetscenesData))
  (bind _returnvalue_2 (Actor|GetComponentbyClass _returnvalue "/Game/Inventory/BP_inventoryComp.BP_inventoryComp_C"))
  (bind _booksheld (Variables|/Game/Inventory/BP_inventoryComp.BP_inventoryComp_C|GetbooksHeld _returnvalue_2))
  (bind _returnvalue_3 (+ _memoriesseen _booksheld -1 1))
  (Default|SetinScene (Variables|Default|Getplayer) true)
  (Variables|Default|SetlastPlayerPosition (Transformation|GetActorTransform _returnvalue))
  (Transformation|SetActorLocation _returnvalue "0.000000,0.000000,999.000000" false true)
  (bind _outrownames (DataTable|GetDataTableRowNames _scenesdata))
  (if (Utilities|Array|IsValidIndex _outrownames _returnvalue_3)
    (bind _returnvalue_4 (Utilities|GetDataTableRow _scenesdata (Utilities|Array|Get(acopy) _outrownames _returnvalue_3))
      (:then
        (Variables|Default|SetcurrentScene (Utilities|Struct|BreakF_imageDialogueArray _returnvalue_4))
        (Variables|Default|SetcurrentSceneCoindices (Utilities|Struct|MakeIntPoint 0 0))
        (CallFunction|FadeinScene)))
    (else
      (Development|PrintString "Hello")
      (CallFunction|EndScene))))

(fn CycleScene
  (if (>= (Utilities|Array|LastIndex (Variables|Default|GetcurrentScene)) (.x (Variables|Default|GetcurrentSceneCoindices)))
    (Audio|SpawnSound2D "/Game/MatsFolder/DialogueAudio/MSS_SpeakingAudio.MSS_SpeakingAudio" 1.0 1.0 0.0 0)
    (Default|CheckUpdateScene (Variables|Default|Getwidget) (.image (Utilities|Array|Get(acopy) (Variables|Default|GetcurrentScene) (.x (Variables|Default|GetcurrentSceneCoindices)))) (Utilities|Array|Get(acopy) (.strings (.dialogue (Utilities|Array|Get(acopy) (Variables|Default|GetcurrentScene) (.x (Variables|Default|GetcurrentSceneCoindices))))) (.y (Variables|Default|GetcurrentSceneCoindices))))
    (if (== (Utilities|Array|LastIndex (.strings (.dialogue (Utilities|Array|Get(acopy) (Variables|Default|GetcurrentScene) (.x (Variables|Default|GetcurrentSceneCoindices)))))) (.y (Variables|Default|GetcurrentSceneCoindices)))
      (bind _output_get (Variables|Default|SetcurrentSceneCoindices (Utilities|Struct|MakeIntPoint (.x (+ (stale _output_get) (Utilities|Struct|MakeIntPoint 1 0))) 0)))
      (else
        (bind _output_get_2 (Variables|Default|SetcurrentSceneCoindices (+ (stale _output_get_2) (Utilities|Struct|MakeIntPoint 0 1))))))
    (else
      (CallFunction|EndScene))))

(fn EndScene
  (if (== (Variables|Default|GetmemoriesSeen) 5)
    (Game|OpenLevel(byObjectReference) "/Game/mainMenu/LVL_mainMenu.LVL_mainMenu")
    (else
      (Default|SetinScene (Variables|Default|Getplayer) false)
      (Transformation|SetActorTransform (Game|GetPlayerCharacter 0) (Variables|Default|GetlastPlayerPosition) false true)
      (Widget|RemovefromParent (Variables|Default|Getwidget))
      (if (Variables|Default|Getstarting)
        (Variables|Default|Setstarting false)
        (Sequencer|Player|CreateLevelSequencePlayer "/Game/levelSqnc/LS_intro.LS_intro" (Utilities|Struct|MakeMovieSceneSequencePlaybackSettings true (Utilities|Struct|MakeMovieSceneSequenceLoopCount 0) "(TickIntervalSeconds=0.000000,EvaluationBudgetMicroseconds=0.000000,bTickWhenPaused=False,bAllowRounding=True)" 1.0 0.0 false false false true true false "None" false))
        (CallFunction|UnhideHud)))))

(fn Start
  (bind _scenesdata (Variables|Default|GetscenesData))
  (Variables|Default|Setstarting true)
  (Default|SetinScene (Variables|Default|Getplayer) true)
  (bind _outrownames (DataTable|GetDataTableRowNames _scenesdata))
  (bind _returnvalue (Utilities|GetDataTableRow _scenesdata (Utilities|Array|Get(acopy) _outrownames))
    (:then
      (Variables|Default|SetcurrentScene (Utilities|Struct|BreakF_imageDialogueArray _returnvalue))
      (Variables|Default|SetcurrentSceneCoindices (Utilities|Struct|MakeIntPoint 0 0))
      (UserInterface|Viewport|AddtoViewport (Variables|Default|Getwidget) 0)
      (CallFunction|CycleScene))))

(fn End
  (bind _scenesdata (Variables|Default|GetscenesData))
  (Default|SetinScene (Variables|Default|Getplayer) true)
  (bind _outrownames (DataTable|GetDataTableRowNames _scenesdata))
  (bind _returnvalue (Utilities|GetDataTableRow _scenesdata (Utilities|Array|Get(acopy) _outrownames 6))
    (:then
      (Variables|Default|SetcurrentScene (Utilities|Struct|BreakF_imageDialogueArray _returnvalue))
      (Variables|Default|SetcurrentSceneCoindices (Utilities|Struct|MakeIntPoint 0 0))
      (UserInterface|Viewport|AddtoViewport (Variables|Default|Getwidget) 0)
      (CallFunction|CycleScene))))

(fn GetBooksIndicator)