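; BP_compassComp is a component for BP_compassActor, meant to give a compass world-yaw directions from the player toward a bookshelf and the next memory book.
; Setup finds the player and bookshelf, registers with the compass maze and caches its owner; ReportNewBook stores the target book.
; UpdateParent passes yaws to the owner, with book yaw intended to snap to 45-degree steps.
; The Setup and UpdateParent calls and both look-at calculations are disconnected.
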(event EventBeginPlay)

(event EventTick
  (params (DeltaSeconds :type Float%20%28single-precision%29)))

(event EventReportNewBook
  (params (newBook :type Actor%20Object%20Reference))
  (Variables|Default|SetnextBook newBook))

(fn UpdateParent
  (Utilities|IsValid (Variables|Default|GetnextBook)
    (:Is%20Valid
      (bind _output_get (LocalVariables|SetnextBookYaw (Utilities|PlayertoNextBook))))
    (:Is%20Not%20Valid
      _))
  (Default|Update (Variables|Default|GetparentActor) (Utilities|PlayertoBookshelf) _output_get))

(fn Setup
  (Variables|Default|Setplayer (Game|Player|GetPlayerPawn 0))
  (bind _outactors (Actor|GetAllActorswithInterface "/Game/memoryBook/IF_bookshelf.IF_bookshelf_C"))
  (Variables|Default|Setbookshelf (Utilities|Array|Get(acopy) _outactors))
  (bind _outactors_2 (Actor|GetAllActorswithInterface "/Game/memoryBook/IF_compassMaze.IF_compassMaze_C"))
  (Class|IFCompassMaze|ReportCompass(Message) (Utilities|Array|Get(acopy) _outactors_2) self)
  (bind _asbp_compass_actor (Utilities|Casting|CastToBP_compassActor (Components|GetOwner)))
  (Variables|Default|SetparentActor _asbp_compass_actor))