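; BP_centralBookshelf is the central bookshelf in the memory book feature, where the player deposits collected books.
; On TryInteract it sends SaveAllBooksMessage to the player pawn and gets back a book count.
; For each book it advances the Saved counter and reveals the matching one of four scene components with its children, skipping invalid indices.
; It returns true only when the count is non-zero.
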(fn ConstructionScript)

(fn TryInteract
  (bind _scene1 (Variables|Default|GetScene1))
  (bind _scene2 (Variables|Default|GetScene2))
  (bind _scene3 (Variables|Default|GetScene3))
  (bind _scene (Variables|Default|GetScene))
  (bind _array (Utilities|Array|MakeArray _scene _scene1 _scene2 _scene3))
  (bind _held (Class|IFBooks|SaveAllBooks(Message) (Game|Player|GetPlayerPawn 0)))
  (if (Math|Conversions|ToBoolean(Integer) _held)
    (for _index (range 0 (- _held 1))
      (bind _result (Math|Integer|IncrementInt (Variables|Default|Getsaved))
        (:%20%20
          (if (Utilities|Array|IsValidIndex _array _result)
            (Rendering|SetVisibility (Utilities|Array|Get(acopy) _array _result) true true)))))
    (return true)
    (else
      (return false))))