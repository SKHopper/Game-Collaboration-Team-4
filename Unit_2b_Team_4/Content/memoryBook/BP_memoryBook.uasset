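; BP_memoryBook is a collectible book that the player picks up by interacting with it.
; On BeginPlay it sums the saved ability total and held book count from the player's inventory component to choose one of five book materials for all mesh slots.
; Interacting sends a transfer-book message to the player pawn, reports the pickup to its parent spawner and destroys the actor.
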(event EventBeginPlay
  (bind _returnvalue (Game|GetPlayerCharacter 0))
  (bind _collectiblebook (Variables|Default|Getcollectiblebook))
  (bind _returnvalue_2 (Actor|GetComponentbyClass _returnvalue "/Game/Inventory/BP_inventoryComp.BP_inventoryComp_C"))
  (bind _total (Default|AbilityTotal (Variables|/Game/Inventory/BP_inventoryComp.BP_inventoryComp_C|GetbookAbilitySaveComponent _returnvalue_2)))
  (Rendering|Material|SetMaterial _collectiblebook 0 (Utilities|Array|Get(acopy) (Utilities|Array|MakeArray "/Game/ASSET/Memory_Books/Book_1_Magenta/M_book1.M_book1" "/Game/ASSET/Memory_Books/Book_2_Cyan/M_book2.M_book2" "/Game/ASSET/Memory_Books/Book_3_Blue/M_book3.M_book3" "/Game/ASSET/Memory_Books/Book_4_Yellow/M_book4.M_book4" "/Game/ASSET/Memory_Books/Book_5_Red/M_book5.M_book5") (+ _total (Variables|/Game/Inventory/BP_inventoryComp.BP_inventoryComp_C|GetbooksHeld _returnvalue_2))))
  (Rendering|Material|SetMaterial _collectiblebook 1 (Utilities|Array|Get(acopy) (Utilities|Array|MakeArray "/Game/ASSET/Memory_Books/Book_1_Magenta/M_book1.M_book1" "/Game/ASSET/Memory_Books/Book_2_Cyan/M_book2.M_book2" "/Game/ASSET/Memory_Books/Book_3_Blue/M_book3.M_book3" "/Game/ASSET/Memory_Books/Book_4_Yellow/M_book4.M_book4" "/Game/ASSET/Memory_Books/Book_5_Red/M_book5.M_book5") (+ _total (Variables|/Game/Inventory/BP_inventoryComp.BP_inventoryComp_C|GetbooksHeld _returnvalue_2))))
  (Rendering|Material|SetMaterial _collectiblebook 2 (Utilities|Array|Get(acopy) (Utilities|Array|MakeArray "/Game/ASSET/Memory_Books/Book_1_Magenta/M_book1.M_book1" "/Game/ASSET/Memory_Books/Book_2_Cyan/M_book2.M_book2" "/Game/ASSET/Memory_Books/Book_3_Blue/M_book3.M_book3" "/Game/ASSET/Memory_Books/Book_4_Yellow/M_book4.M_book4" "/Game/ASSET/Memory_Books/Book_5_Red/M_book5.M_book5") (+ _total (Variables|/Game/Inventory/BP_inventoryComp.BP_inventoryComp_C|GetbooksHeld _returnvalue_2))))
  (Rendering|Material|SetMaterial _collectiblebook 3 (Utilities|Array|Get(acopy) (Utilities|Array|MakeArray "/Game/ASSET/Memory_Books/Book_1_Magenta/M_book1.M_book1" "/Game/ASSET/Memory_Books/Book_2_Cyan/M_book2.M_book2" "/Game/ASSET/Memory_Books/Book_3_Blue/M_book3.M_book3" "/Game/ASSET/Memory_Books/Book_4_Yellow/M_book4.M_book4" "/Game/ASSET/Memory_Books/Book_5_Red/M_book5.M_book5") (+ _total (Variables|/Game/Inventory/BP_inventoryComp.BP_inventoryComp_C|GetbooksHeld _returnvalue_2))))
  (Rendering|Material|SetMaterial _collectiblebook 4 (Utilities|Array|Get(acopy) (Utilities|Array|MakeArray "/Game/ASSET/Memory_Books/Book_1_Magenta/M_book1.M_book1" "/Game/ASSET/Memory_Books/Book_2_Cyan/M_book2.M_book2" "/Game/ASSET/Memory_Books/Book_3_Blue/M_book3.M_book3" "/Game/ASSET/Memory_Books/Book_4_Yellow/M_book4.M_book4" "/Game/ASSET/Memory_Books/Book_5_Red/M_book5.M_book5") (+ _total (Variables|/Game/Inventory/BP_inventoryComp.BP_inventoryComp_C|GetbooksHeld _returnvalue_2))))
  (Rendering|Material|SetMaterial _collectiblebook 5 (Utilities|Array|Get(acopy) (Utilities|Array|MakeArray "/Game/ASSET/Memory_Books/Book_1_Magenta/M_book1.M_book1" "/Game/ASSET/Memory_Books/Book_2_Cyan/M_book2.M_book2" "/Game/ASSET/Memory_Books/Book_3_Blue/M_book3.M_book3" "/Game/ASSET/Memory_Books/Book_4_Yellow/M_book4.M_book4" "/Game/ASSET/Memory_Books/Book_5_Red/M_book5.M_book5") (+ _total (Variables|/Game/Inventory/BP_inventoryComp.BP_inventoryComp_C|GetbooksHeld _returnvalue_2)))))

(fn ConstructionScript)

(fn GetPickedUp
  (Class|IFBooks|TransferBook(Message) (Game|Player|GetPlayerPawn 0))
  (Default|ReportBookPickedUp (Variables|Default|GetparentSpawner))
  (Actor|DestroyActor))

(fn TryInteract
  (CallFunction|GetPickedUp)
  (return true))