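; Inventory component that tracks the player's saved book count as ability progression.
; Each TransferBook event increments the count and passes it to the memory scene component to update memories seen.
; The first and second books trigger floor-draw and trap messages on the player pawn, while invisibility, throwing-distraction and moving-cart messages are unwired.
; AbilityTotal returns the count; GetBookComponent and SaveAllBooks are empty stubs.
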(event EventTransferBook
  (CallFunction|IncrementProgression))

(fn IncrementProgression
  (bind _returnvalue (Game|Player|GetPlayerPawn 0))
  (bind _result (Math|Integer|IncrementInt (Variables|Default|GetbooksSaved))
    (:%20%20
      (Default|UpdateMemoriesSeen (Variables|Default|GetmemorySceneComp) _result)
      (switch int _result
        (:1
          (Class|IFInventory|ActivateFloorDraw(Message) _returnvalue))
        (:2
          (Class|IFInventory|ActivateTrap(Message) _returnvalue))))))

(fn AbilityTotal
  (return (Variables|Default|GetbooksSaved)))

(fn GetBookComponent
  (return 0))

(fn SaveAllBooks
  (return 0))