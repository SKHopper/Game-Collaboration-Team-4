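; Player inventory component that opens and closes the inventory screen and tracks the books the player is carrying.
; It creates the inventory widget on BeginPlay and, when toggled, switches input mode and cursor and disables or restores character movement.
; Picked-up books update the widget and notify the memory scene component.
; Saving transfers books to the book ability component, fetched through owner interfaces, and shows each new ability in the widget.
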(event EventInventoryToggle
  (CallFunction|ToggleInventory))

(event EventTransferBook
  (CallFunction|ChangeBooksHeld 1)
  (Default|BookPickedUp (Variables|Default|GetmemorySceneComp)))

(event EventBeginPlay
  (CallFunction|Setup))

(event EventOpenInventory
  (CallFunction|ActivateInventory))

(event EventCloseInventory
  (CallFunction|DeactivateInventory))

(event EventReset
  (CallFunction|ResetBooksHeld))

(fn MakeInventoryWidget
  (bind _returnvalue (UserInterface|CreateWidget "/Game/Inventory/WBP_inventory.WBP_inventory_C" 0 self))
  (Variables|Default|SetinventoryWidget _returnvalue))

(fn Setup
  (CallFunction|MakeInventoryWidget)
  (bind _asif_inventory (Utilities|Casting|CastToIF_inventory (Components|GetOwner)))
  (bind _output_get (Variables|Default|SetplayerForInventory _asif_inventory))
  (bind _asif_books (Utilities|Casting|CastToIF_books _output_get))
  (bind _output_get_2 (Variables|Default|SetplayerForBooks _asif_books))
  (bind _comp (Default|GetBookComponent _output_get_2))
  (Variables|Default|SetbookAbilitySaveComponent _comp)
  (Input|SetInputModeGameOnly (Game|GetPlayerController 0) false))

(fn ActivateInventory
  (bind _returnvalue (Game|GetPlayerController 0))
  (bind _inventorywidget (Variables|Default|GetinventoryWidget))
  (Variables|/Script/Engine.PlayerController|SetbShowMouseCursor _returnvalue true)
  (Input|SetInputModeUIOnly _returnvalue _inventorywidget "DoNotLock" false)
  (UserInterface|Viewport|AddtoViewport _inventorywidget 0)
  (Default|OpenInventory _inventorywidget)
  (Pawn|Components|CharacterMovement|DisableMovement (Variables|/Script/Engine.Character|GetCharacterMovement (Game|GetPlayerCharacter 0))))

(fn DeactivateInventory
  (bind _returnvalue (Game|GetPlayerController 0))
  (bind _inventorywidget (Variables|Default|GetinventoryWidget))
  (Variables|/Script/Engine.PlayerController|SetbShowMouseCursor _returnvalue false)
  (Input|SetInputModeGameOnly _returnvalue false)
  (Widget|RemovefromParent _inventorywidget)
  (Default|CloseInventory _inventorywidget)
  (Pawn|Components|CharacterMovement|SetMovementMode (Variables|/Script/Engine.Character|GetCharacterMovement (Game|GetPlayerCharacter 0)) "MOVE_Falling" 0))

(fn ToggleInventory
  (if (Variables|Default|GetisOpen)
    (Variables|Default|SetisOpen false)
    (CallFunction|CloseInventory)
    (else
      (Variables|Default|SetisOpen true)
      (CallFunction|OpenInventory))))

(fn ChangeBooksHeld
  (params (delta :type Integer))
  (bind _output_get (Variables|Default|SetbooksHeld (+ delta (Variables|Default|GetbooksHeld))))
  (Default|SetBooksHeld (Variables|Default|GetinventoryWidget) _output_get))

(fn SaveABook
  (if (Math|Conversions|ToBoolean(Integer) (Variables|Default|GetbooksHeld))
    (Default|TransferBook (Variables|Default|GetbookAbilitySaveComponent))
    (CallFunction|ChangeBooksHeld -1)
    (bind _total (Default|AbilityTotal (Variables|Default|GetbookAbilitySaveComponent)))
    (Default|NewAbility (Variables|Default|GetinventoryWidget) (- _total 1))))

(fn ResetBooksHeld
  (CallFunction|ChangeBooksHeld (- 0 (Variables|Default|GetbooksHeld))))

(fn AbilityTotal)

(fn GetBookComponent
  (return 0))

(fn SaveAllBooks
  (bind _booksheld (Variables|Default|GetbooksHeld))
  (bind _returnvalue (Math|Conversions|ToBoolean(Integer) _booksheld))
  (bind _output_get (LocalVariables|Settemp _booksheld))
  (if _returnvalue
    (while _returnvalue
      (CallFunction|SaveABook))
    (return _output_get)
    (else
      (return 0))))