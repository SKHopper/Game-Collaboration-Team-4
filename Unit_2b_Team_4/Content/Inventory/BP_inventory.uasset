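; Inventory component that shows and hides the inventory UI for the actor that owns it.
; On BeginPlay it creates a WBP_inventory widget and stores the owner through the IF_inventory interface.
; A toggle event flips IsOpen and fires open or close events, which add or remove the widget, call its own open/close functions, and switch player 0's cursor and input mode.
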(event EventInventoryToggle
  (CallFunction|ToggleInventory))

(event EventBeginPlay
  (CallFunction|Setup))

(event EventOpenInventory
  (CallFunction|ActivateInventory))

(event EventCloseInventory
  (CallFunction|DeactivateInventory))

(fn MakeInventoryWidget
  (bind _returnvalue (UserInterface|CreateWidget "/Game/Inventory/WBP_inventory.WBP_inventory_C" 0 self))
  (Variables|Default|SetinventoryWidget _returnvalue))

(fn Setup
  (CallFunction|MakeInventoryWidget)
  (bind _asif_inventory (Utilities|Casting|CastToIF_inventory (Components|GetOwner)))
  (Variables|Default|Setplayer _asif_inventory))

(fn ActivateInventory
  (bind _returnvalue (Game|GetPlayerController 0))
  (bind _inventorywidget (Variables|Default|GetinventoryWidget))
  (Variables|/Script/Engine.PlayerController|SetbShowMouseCursor _returnvalue true)
  (Input|SetInputModeGameandUI _returnvalue _inventorywidget "DoNotLock" true false)
  (UserInterface|Viewport|AddtoViewport _inventorywidget 0)
  (Default|OpenInventory _inventorywidget))

(fn DeactivateInventory
  (bind _returnvalue (Game|GetPlayerController 0))
  (bind _inventorywidget (Variables|Default|GetinventoryWidget))
  (Variables|/Script/Engine.PlayerController|SetbShowMouseCursor _returnvalue false)
  (Input|SetInputModeGameOnly _returnvalue false)
  (Widget|RemovefromParent _inventorywidget)
  (Default|CloseInventory _inventorywidget))

(fn ToggleInventory
  (if (Variables|Default|GetisOpen)
    (Variables|Default|SetisOpen false)
    (CallFunction|CloseInventory)
    (else
      (Variables|Default|SetisOpen true)
      (CallFunction|OpenInventory))))