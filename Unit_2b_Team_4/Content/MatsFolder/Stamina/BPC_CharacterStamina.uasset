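; Character stamina component that drives sprinting, with a stamina bar widget created on BeginPlay.
; Sprint needs over a fifth of max stamina, raises walk speed and FOV, and starts a looping drain timer.
; Stop restores both and starts a looping regen timer that clears at full stamina.
; Both timers feed UpdateStamina, which clamps the value and updates the widget; reaching zero does not stop sprinting.
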(event Custom|EndRegen
  (Utilities|Time|ClearandInvalidateTimerbyHandle (Variables|Default|GetTimerRef)))

(event Custom|stop
  (Utilities|Time|ClearandInvalidateTimerbyHandle (Variables|Default|GetsprintTickTimer))
  (Variables|/Script/Engine.CharacterMovementComponent|SetMaxWalkSpeed (Variables|/Script/Engine.Character|GetCharacterMovement (Game|GetPlayerCharacter 0)) (Variables|Default|GetwalkSpeed))
  (Default|ScaleFov (Variables|Default|GetcamFov) 9e+01)
  (Variables|Default|SetIsSprinting false)
  (bind _returnvalue (Utilities|Time|SetTimerbyFunctionName 0 "RegenStamina" (Variables|Default|GetRegenRate) true))
  (Variables|Default|SetTimerRef _returnvalue))

(event Custom|Sprint
  (if (> (Variables|Default|GetStamina) (/ (Variables|Default|GetMaxStamina) 5.0))
    (Variables|Default|SetIsSprinting true)
    (Default|ScaleFov (Variables|Default|GetcamFov) 105.0)
    (Variables|/Script/Engine.CharacterMovementComponent|SetMaxWalkSpeed (Variables|/Script/Engine.Character|GetCharacterMovement (Game|GetPlayerCharacter 0)) (Variables|Default|GetsprintSpeed))
    (bind _returnvalue (Utilities|Time|SetTimerbyEvent (delegate Custom|sprintTick) 0.1 true))
    (Variables|Default|SetsprintTickTimer _returnvalue)))

(event Custom|sprintTick
  (CallFunction|UpdateStamina -0.3))

(event EventBeginPlay
  (bind _returnvalue (UserInterface|CreateWidget "/Game/MatsFolder/WBP_sprint.WBP_sprint_C"))
  (bind _output_get (Variables|Default|Setwidget _returnvalue))
  (UserInterface|Viewport|AddtoViewport _output_get 0)
  (Variables|Default|SetwalkSpeed (Variables|/Script/Engine.CharacterMovementComponent|GetMaxWalkSpeed (Variables|/Script/Engine.Character|GetCharacterMovement (Game|GetPlayerCharacter 0)))))

(fn RegenStamina
  (CallFunction|UpdateStamina 0.1)
  (if (== (Variables|Default|GetStamina) (Variables|Default|GetMaxStamina))
    (CallFunction|EndRegen)))

(fn UpdateStamina
  (params (delta :type Float%20%28double-precision%29))
  (bind _output_get (Variables|Default|SetStamina (Math|Float|Clamp(Float) (+ delta (Variables|Default|GetStamina)) 0.0 (Variables|Default|GetMaxStamina))))
  (Default|UpdateStamina (Variables|Default|Getwidget) (/ _output_get (Variables|Default|GetMaxStamina)))
  (if (== (Variables|Default|GetStamina) 0.0)
    _))