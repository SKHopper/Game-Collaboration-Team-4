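; Trap component that lets the player place salt traps at their feet, gated by an unlock flag and a full trap bar.
; CreateTrap freezes the player's walk speed during a short placement delay, empties the bar, spawns BP_SaltTrap and destroys the oldest once the count exceeds the limit.
; Execute calls CreateTrap, then after a delay starts a looping TrapRegen timer that refills the bar and stops when full.
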(event Custom|CreateTrap
  (bind _traps (Variables|Default|Gettraps))
  (bind _playerref (Variables|Default|GetPlayerRef))
  (bind _output (Utilities|Array|Get(acopy) _traps))
  (bind _charactermovement (Variables|/Script/Engine.Character|GetCharacterMovement _playerref))
  ;[0.15 0.15 0.15 0.5] creates the trap and stops the player moving while they place it under them
  (if (stale EventActivateTrap _output_get)
    (if (== (Variables|Default|GetTrapBarAmount) (Variables|Default|GetMaxTrapBar))
      (if (< (Variables|Default|GetmaxTrapCount) (Utilities|Array|Length (Variables|Default|Gettraps)))
        (Utilities|IsValid _output
          (:Is%20Valid
            (Actor|DestroyActor _output))
          (:Is%20Not%20Valid
            _))
        (Utilities|Array|RemoveIndex _traps))
      (Variables|/Script/Engine.CharacterMovementComponent|SetMaxWalkSpeed _charactermovement 0.0)
      (Utilities|FlowControl|Delay 2.5)
      (Variables|/Script/Engine.CharacterMovementComponent|SetMaxWalkSpeed _charactermovement 6e+02)
      (Variables|Default|SetTrapBarAmount 0.0)
      (bind _returnvalue (Game|SpawnActorfromClass "/Game/MatsFolder/Traps/BP_SaltTrap.BP_SaltTrap_C" (Math|Conversions|ToTransform(Vector) (- (Transformation|GetWorldLocation (Variables|/Script/Engine.Actor|GetRootComponent (Game|GetPlayerCharacter 0))) "0.000000,0.000000,97.649994")) "Undefined" "MultiplyWithRoot" 0 self 0))
      (Utilities|Array|Add (Variables|Default|Gettraps) _returnvalue))))

(event Custom|Regenerate%20Trap
  (bind _returnvalue (Utilities|Time|SetTimerbyFunctionName 0 "TrapRegen" 0.5 true))
  (Variables|Default|SetTrap%20Timer%20Handle _returnvalue)
  (Development|PrintString (Utilities|String|ToString(Float) (Variables|Default|GetTrapBarAmount))))

(event Custom|EndTrapRegen
  (Utilities|Time|ClearandInvalidateTimerbyHandle (Variables|Default|GetTrap%20Timer%20Handle)))

(event Custom|Execute
  (CallFunction|CreateTrap)
  (Utilities|FlowControl|Delay 2.6)
  (CallFunction|RegenerateTrap))

(event EventBeginPlay
  (bind _returnvalue (Actor|GetActorOfClass "/Game/FirstPerson/Blueprints/BP_FirstPersonCharacter.BP_FirstPersonCharacter_C"))
  (Variables|Default|SetPlayerRef _returnvalue))

(event EventActivateTrap
  (bind _output_get (Variables|Default|SetcanTrap true)))

(fn TrapRegen
  (Variables|Default|SetTrapBarAmount (Math|Float|Clamp(Float) (+ (Variables|Default|GetTrapBarAmount) 0.5) 0.0 (Variables|Default|GetMaxTrapBar)))
  (Development|PrintString (Utilities|String|ToString(Float) (Variables|Default|GetTrapBarAmount)))
  (if (== (Variables|Default|GetTrapBarAmount) (Variables|Default|GetMaxTrapBar))
    (CallFunction|EndTrapRegen)))