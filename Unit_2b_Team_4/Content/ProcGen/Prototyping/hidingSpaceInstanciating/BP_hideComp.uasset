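; BP_hideComp is a prototype component that puts the first-person player into and out of hiding spaces.
; On BeginPlay it caches the player character; entering stores the hide object, disables movement and sets the Hidden flag.
; Leaving clears the flag, restores movement in Falling mode, then reattaches the camera to the first-person mesh at its relative offset from the player.
; Leave attempts are delegated to the stored hide object; GetCam is an empty stub.
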(event Custom|tryLeaveHide
  (Default|LeaveHide (Variables|Default|Gethide)))

(event EventBeginPlay
  (bind _asbp_first_person_character (Utilities|Casting|CastToBP_FirstPersonCharacter (Game|Player|GetPlayerPawn 0)))
  (Variables|Default|Setplayer _asbp_first_person_character))

(event EventEntreHide
  (params (hide :type IF%20Hide%20Interface))
  (Variables|Default|Sethide hide)
  (Pawn|Components|CharacterMovement|DisableMovement (Variables|/Script/Engine.Character|GetCharacterMovement (Variables|Default|Getplayer)))
  (Variables|Default|Sethidden true))

(event EventLeaveHide
  (bind _player (Variables|Default|Getplayer))
  (bind _player_2 (Variables|Default|Getplayer))
  (bind _firstpersoncameracomponent (Variables|/Script/Unit_2b_Team_4.Unit_2b_Team_4Character|GetFirstPersonCameraComponent _player_2))
  (Variables|Default|Sethidden false)
  (Pawn|Components|CharacterMovement|SetMovementMode (Variables|/Script/Engine.Character|GetCharacterMovement _player_2) "MOVE_Falling" 0)
  (Transformation|AttachComponentToComponent _firstpersoncameracomponent (Variables|/Script/Unit_2b_Team_4.Unit_2b_Team_4Character|GetFirstPersonMesh _player_2) "None" "KeepWorld" "KeepRelative" "KeepRelative" true)
  (Transformation|SetWorldLocation _firstpersoncameracomponent (+ (Variables|/Game/FirstPerson/Blueprints/BP_FirstPersonCharacter.BP_FirstPersonCharacter_C|GetcameraRelative _player) (Transformation|GetActorLocation _player)) false false))

(fn GetCam
  (return 0))