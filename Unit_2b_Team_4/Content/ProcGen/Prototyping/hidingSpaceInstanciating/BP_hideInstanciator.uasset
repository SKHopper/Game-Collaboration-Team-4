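; BP_hideInstanciator manages procedurally placed bookshelf hiding spots, loading and unloading them with the world grid.
; A weighted roll picks hide spots, whose wall-side transforms are saved per large grid cell, using the parent manager's wall offsets.
; Saved spots spawn as a randomly big or regular custom ISM instance paired with a BP_hideSpace actor.
; Unloading a cell removes those instances and actors but keeps the saved transforms.
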(fn GenerateIsNotHide
  (return (not (Math|Random|RandomBoolwithWeight (Variables|Default|GetweightBookshelfIsHideSpot)))))

(fn SaveHide
  (params (in :type F%20Point%20Wall%20Structure))
  (bind _largegridsides (Variables|Default|GetlargeGridSides))
  (bind _transform (CallFunction|GetTransform (.sideindex in) (.world in)))
  (Utilities|Array|Add (Variables|Default|Getsaved) _transform)
  (if (Utilities|Map|Contains (Variables|Default|GetlargeGridSides) (.world in))
    _
    (else
      (Utilities|Map|Add _largegridsides (.world in) (Utilities|Struct|MakeF_transformArray (Utilities|Array|MakeArray)))))
  (bind _output_get (LocalVariables|Settemp (.transforms (.Value (Utilities|Map|Find _largegridsides (.world in))))))
  (Utilities|Array|Add _output_get _transform)
  (Utilities|Map|Add (Variables|Default|GetlargeGridSides) (.world in) (Utilities|Struct|MakeF_transformArray _output_get)))

(fn CheckInstanciateHide
  (params (in :type F%20Point%20Wall%20Structure))
  (bind _transform (CallFunction|GetTransform (.sideindex in) (.world in)))
  (if (Utilities|Array|ContainsItem (Variables|Default|Getsaved) _transform)
    (CallFunction|SpawnHide _transform)))

(fn GetTransform
  (params (index :type Integer) (world :type Vector%202D%20Structure))
  (bind _worldoffset (Default|CalcWallOffset (Variables|Default|GetparentManager) index))
  (return (Math|Transform|MakeTransform (+ _worldoffset world) (Math|Rotator|CombineRotators "0.000000,0.000000,90.000000" (Math|Rotator|CombineRotators "0.000000,90.000000,0.000000" (Math|Rotator|MakeRotator 0.0 0.0 (Math|Conversions|ToFloat(Integer) (* index 90))))))))

(fn SpawnHide
  (params (InstanceTransform :type Transform%20%28by%20ref%29))
  (bind _returnvalue (Math|Random|RandomBool))
  (bind _output_get (LocalVariables|Setbig _returnvalue))
  (Utilities|Map|Add (Variables|Default|GetbigHides) InstanceTransform _returnvalue)
  (Default|AddInstanceCustom (select _output_get (Variables|Default|GetcustomISMBig) (Variables|Default|GetcustomISM)) InstanceTransform true)
  (bind _returnvalue_2 (Game|SpawnActorfromClass "/Game/ProcGen/Prototyping/hidingSpaceInstanciating/BP_hideSpace.BP_hideSpace_C" (Math|Transform|MakeTransform (.location InstanceTransform) (Math|Rotator|CombineRotators "0.000000,0.000000,-90.000000" (.rotation InstanceTransform)) (.scale InstanceTransform)) "AlwaysSpawn" "MultiplyWithRoot" 0 (LocalVariables|Getbig) 0))
  (Utilities|Map|Add (Variables|Default|GetloadedSpaces) InstanceTransform _returnvalue_2))

(fn CheckUninstanciateHide
  (params (largeGrid :type Vector%202D%20Structure%20%28by%20ref%29))
  (bind _customism (Variables|Default|GetcustomISM))
  (for _array_element (.transforms (.Value (Utilities|Map|Find (Variables|Default|GetlargeGridSides) largeGrid)))
    (Utilities|IsValid (.Value (Utilities|Map|Find (Variables|Default|GetloadedSpaces) _array_element))
      (:Is%20Valid
        (Actor|DestroyActor (.Value (Utilities|Map|Find (Variables|Default|GetloadedSpaces) _array_element))))
      (:Is%20Not%20Valid
        _))
    (bind _instanceindex (Default|FindInstanceIndex _customism (.Location (Math|Transform|BreakTransform _array_element))))
    (Default|RemoveInstanceCustom (select (.Value (Utilities|Map|Find (Variables|Default|GetbigHides) _array_element)) (Variables|Default|GetcustomISMBig) _customism) _instanceindex)))