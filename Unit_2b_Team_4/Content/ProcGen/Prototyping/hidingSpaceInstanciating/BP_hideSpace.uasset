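; Interactable hiding spot Blueprint with pivoting doors that lets the player hide inside and later leave.
; Interacting opens four door pivots with a timeline, then after a short delay saves the player's location and attaches their camera to the nearer of two camera points.
; The pawn is parked at the world origin while hidden and teleported back on leave.
; A second timeline drives partial door opening for the hidden state and exit.
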(event Custom|lerpDoors
  (params (outward :type Boolean))
  (if outward
    (bind _floatcurvedoors (Timeline|TL_doors PlayFromStart)
      (:Update
        (CallFunction|RotationTick _floatcurvedoors)))
    (else
      (Timeline|TL_doors ReverseFromEnd))))

(event Custom|lerpDoorsPartial
  (params (outward :type Boolean))
  (if outward
    (bind _curve2 (Timeline|TL_partialDoors PlayFromStart)
      (:Update
        (CallFunction|RotationTick _curve2)))
    (else
      (Timeline|TL_partialDoors ReverseFromEnd))))

(event Custom|entre
  (CallFunction|LerpDoors true)
  (Utilities|FlowControl|Delay 0.6)
  (CallFunction|MoveInside))

(event EventLeaveHide
  (CallFunction|LerpDoorsPartial true)
  (Utilities|FlowControl|Delay 0.6)
  (CallFunction|MoveOutside))

(fn ConstructionScript)

(fn RotationTick
  (params (lerpAlpha :type Float%20%28single-precision%29))
  (for (_array_element _array_index) (Utilities|Array|MakeArray (Variables|Default|GetpivotL1) (Variables|Default|GetpivotR1) (Variables|Default|GetpivotL2) (Variables|Default|GetpivotR2))
    (Transformation|SetRelativeRotation _array_element (Math|Rotator|Lerp(Rotator) "0, 0, 0" (Utilities|Array|Get(acopy) (Variables|Default|GetopenRotations) _array_index) lerpAlpha true) false true)))

(fn Exit
  (CallFunction|LerpDoors false))

(fn MoveInside
  (bind _returnvalue (Game|Player|GetPlayerPawn 0))
  (Class|IFHide|EntreHide(Message) _returnvalue self)
  (bind _cam (Class|IFHide|GetCam(Message) _returnvalue))
  (Variables|Default|SetplayerCam _cam)
  (bind _output_get (Variables|Default|SetplayerLastUnhiddenLocation (Transformation|GetActorLocation _returnvalue)))
  (Transformation|SetWorldTransform (Variables|Default|GetplayerCam) (.out (Utilities|SelectCamScene _output_get)) false true)
  (Transformation|AttachComponentToComponent (Variables|Default|GetplayerCam) (.obj (Utilities|SelectCamScene _output_get)) "None" "KeepWorld" "KeepWorld" "KeepWorld" true)
  (Transformation|SetActorLocation (Game|Player|GetPlayerPawn 0) "0, 0, 0" false true)
  (CallFunction|LerpDoorsPartial false))

(fn MoveOutside
  (Transformation|SetActorLocation (Game|Player|GetPlayerPawn 0) (Variables|Default|GetplayerLastUnhiddenLocation) false true)
  (Class|IFHide|LeaveHide(Message) (Game|Player|GetPlayerPawn 0))
  (CallFunction|LerpDoors false))

(fn GetCam
  (return 0))

(fn TryInteract
  (CallFunction|Entre)
  (return true))