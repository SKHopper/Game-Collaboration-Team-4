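; Prototype nav-tracking component that records which integer grid cells are closed off.
; AddPointsAround writes a 3x3 block of flags around a centre through SetMapValue, which grows nested arrays on demand.
; Storage is split into four quadrant maps indexed by absolute coordinates, but only the positive quadrant is wired; negative cells are skipped.
; A test event draws the positive map as red or green debug circles.
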(event Custom|test
  (for (_array_element _array_index) (Variables|Default|Getmap)
    (for (_array_element_2 _array_index_2) (.membervar_0 _array_element)
      (Rendering|Debug|DrawDebugCircle (Math|Vector|MakeVector (.x (/ (* (Math|Vector|MakeVector (Math|Conversions|ToFloat(Integer) _array_index) (Math|Conversions|ToFloat(Integer) _array_index_2) 0.0) 1e+03) 3.0)) (.y (/ (* (Math|Vector|MakeVector (Math|Conversions|ToFloat(Integer) _array_index) (Math|Conversions|ToFloat(Integer) _array_index_2) 0.0) 1e+03) 3.0)) 2e+02) 3e+01 12 (Math|Color|SelectColor "(R=1.000000,G=0.000000,B=0.000000,A=1.000000)" "(R=0.000000,G=1.000000,B=0.000000,A=1.000000)" _array_element_2) 2e+01 2e+01 "0.000000,1.000000,0.000000" "0.000000,0.000000,1.000000"))))

(fn AddPointsAround
  (params (centrePoint :type Int%20Vector%202%20Structure) (points :type Array%20of%20F%20Boolean%20Array%20Structures))
  (bind (_x _y) (Utilities|Struct|BreakIntVector2 centrePoint))
  (bind _xy (LocalVariables|Getxy))
  (for _index (range -1 1)
    (Utilities|Struct|SetmembersinIntVector2 _xy (+ _index _x))
    (for _index_2 (range -1 1)
      (bind _structout (Utilities|Struct|SetmembersinIntVector2 _xy (+ _y _index_2)))
      (CallFunction|SetMapValue _structout (Utilities|Array|Get(acopy) (.membervar_0 (Utilities|Array|Get(acopy) points (+ _index 1))) (+ _index_2 1))))))

(fn SetMapValue
  (params (xy :type Int%20Vector%202%20Structure) (closedOff :type Boolean))
  (bind _returnvalue (> (.y xy) -1))
  (bind _output_get (LocalVariables|SetabsXY (Utilities|Struct|MakeIntVector2 (Math|Integer|Absolute(Integer) (.x xy)) (Math|Integer|Absolute(Integer) (.y xy)))))
  (if (> (.x xy) -1)
    (if _returnvalue
      (bind _output_get_2 (LocalVariables|Setquadrant 0))
      (CallFunction|UpdateMapXSize _output_get_2 (.x (LocalVariables|GetabsXY)))
      (switch int (LocalVariables|Getquadrant)
        (:0
          (Utilities|Array|SetArrayElem (.membervar_0 (Utilities|Array|Get(acopy) (Variables|Default|Getmap) (.x (LocalVariables|GetabsXY)))) (.y (LocalVariables|GetabsXY)) closedOff true))
        (:1
          (Utilities|Array|SetArrayElem (.membervar_0 (Utilities|Array|Get(acopy) (Variables|Default|GetmapNegX) (.x (LocalVariables|GetabsXY)))) (.y (LocalVariables|GetabsXY)) closedOff true))
        (:2
          (Utilities|Array|SetArrayElem (.membervar_0 (Utilities|Array|Get(acopy) (Variables|Default|GetmapNegY) (.x (LocalVariables|GetabsXY)))) (.y (LocalVariables|GetabsXY)) closedOff true))
        (:3
          (Utilities|Array|SetArrayElem (.membervar_0 (Utilities|Array|Get(acopy) (Variables|Default|GetmapNegXY) (.x (LocalVariables|GetabsXY)))) (.y (LocalVariables|GetabsXY)) closedOff true))))
    (elif _returnvalue
      _)))

(fn UpdateMapXSize
  (params (mapQuadrant :type Integer) (x :type Integer))
  (if (not (>= (Utilities|Select :Index mapQuadrant :Option%200 (Utilities|Array|LastIndex (Variables|Default|Getmap)) :Option%201 (Utilities|Array|LastIndex (Variables|Default|GetmapNegX)) :Option%202 (Utilities|Array|LastIndex (Variables|Default|GetmapNegY)) :Option%203 (Utilities|Array|LastIndex (Variables|Default|GetmapNegXY))) x))
    (switch int mapQuadrant
      (:0
        (Utilities|Array|SetArrayElem :TargetArray (Variables|Default|Getmap) :Index x :bSizeToFit true))
      (:1
        (Utilities|Array|SetArrayElem :TargetArray (Variables|Default|GetmapNegX) :Index x :bSizeToFit true))
      (:2
        (Utilities|Array|SetArrayElem :TargetArray (Variables|Default|GetmapNegY) :Index x :bSizeToFit true))
      (:3
        (Utilities|Array|SetArrayElem :TargetArray (Variables|Default|GetmapNegXY) :Index x :bSizeToFit true)))))