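; Candle component for procedurally generated bookshelves, placing candles in free shelf spots.
; GenerateCandleSpot uses a weighted random roll to store each spot's shelf-relative transform as a candle, or track it among that shelf's free spots.
; CheckInstanciate converts stored transforms to world space, spawns BP_candle actors and adds custom ISM instances.
; CheckUninstanciate finds loaded instances by location and removes them, leaving spawned actors untouched.
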(fn GenerateCandleSpot
  (params (bookshelf :type Transform) (spotRelative :type Transform))
  (bind _instances (Variables|Default|Getinstances))
  (bind (_value _returnvalue) (Utilities|Map|Find _instances bookshelf))
  (if (Math|Random|RandomBoolwithWeight (Variables|Default|GetweightFreeSpotIsCandle))
    (if _returnvalue
      (bind _output_get (LocalVariables|Settemp (.transforms _value)))
      (Utilities|Array|Add _output_get spotRelative)
      (Utilities|Map|Add (Variables|Default|Getinstances) bookshelf (Utilities|Struct|MakeF_transformArray (LocalVariables|Gettemp)))
      (else
        (Utilities|Map|Add (Variables|Default|Getinstances) bookshelf (Utilities|Struct|MakeF_transformArray (Utilities|Array|MakeArray spotRelative)))))
    (elif (== (Variables|Default|GetcurrentGeneratingShelf) bookshelf)
      (Utilities|Array|Add (Variables|Default|GetcurrentShelfFreeSpots) spotRelative)
      (else
        (Utilities|Map|Add (Variables|Default|GetfreeSpots) (Variables|Default|GetcurrentGeneratingShelf) (Utilities|Struct|MakeF_transformArray (Variables|Default|GetcurrentShelfFreeSpots)))
        (Variables|Default|SetcurrentGeneratingShelf bookshelf)
        (Utilities|Array|Clear (Variables|Default|GetcurrentShelfFreeSpots))))))

(fn CheckInstanciate
  (params (bookshelf :type Transform))
  (bind _instances (Variables|Default|Getinstances))
  (bind (_value _returnvalue) (Utilities|Map|Find _instances bookshelf))
  (if _returnvalue
    (for _array_element (.transforms _value)
      (Game|SpawnActorfromClass "/Game/ProcGen/Prototyping/bookInstanciating/otherBookshelfItems/BP_candle.BP_candle_C" (Math|Transform|MakeTransform (+ (Math|Vector|RotateVector (.location _array_element) (.rotation bookshelf)) (.location bookshelf)) (Math|Rotator|CombineRotators (.rotation _array_element) (.rotation bookshelf))) "Undefined" "MultiplyWithRoot" 0 0)
      (Default|AddInstanceCustom (Variables|Default|GetcustomISM) (Math|Transform|MakeTransform (+ (Math|Vector|RotateVector (.location _array_element) (.rotation bookshelf)) (.location bookshelf)) (Math|Rotator|CombineRotators (.rotation _array_element) (.rotation bookshelf)) "0.200000,0.200000,0.200000") true)
      (Utilities|Array|Add (LocalVariables|Gettemp) (Math|Transform|MakeTransform (+ (Math|Vector|RotateVector (.location _array_element) (.rotation bookshelf)) (.location bookshelf)) (Math|Rotator|CombineRotators (.rotation _array_element) (.rotation bookshelf)) "0.200000,0.200000,0.200000")))
    (Utilities|Map|Add (Variables|Default|GetloadedInstances) (.location bookshelf) (Utilities|Struct|MakeF_transformArray (LocalVariables|Gettemp)))))

(fn CheckUninstanciate
  (params (bookshelf :type Vector))
  (bind _customism (Variables|Default|GetcustomISM))
  (for _array_element (.transforms (.Value (Utilities|Map|Find (Variables|Default|GetloadedInstances) bookshelf)))
    (bind _instanceindex (Default|FindInstanceIndex _customism (.location _array_element)))
    (Default|RemoveInstanceCustom _customism _instanceindex))
  (Utilities|Map|Remove (Variables|Default|GetloadedInstances) bookshelf))