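; Item pool component that pre-spawns candles and ink bottles for the bookshelf item prototype.
; On BeginPlay it spawns both populations at a far-away transform into separate queues, with all ink bottles sharing one explosion actor and referencing the pool.
; ReportThrown parks the item far away again and moves it to the front of the ink bottle queue.
; Pickup, throw and camera-position functions are stubs.
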(event EventBeginPlay
  (CallFunction|PoolItems))

(event EventReportThrown
  (params (item :type BP%20Ink%20Item%20Object%20Reference))
  (bind _inkbottlequeue (Variables|Default|GetinkBottleQueue))
  (Transformation|SetActorTransform item (Variables|Default|GetfarAway))
  (Utilities|Array|RemoveItem _inkbottlequeue item)
  (Utilities|Array|Insert _inkbottlequeue item))

(fn PoolItems
  (bind _faraway (Variables|Default|GetfarAway))
  (bind _returnvalue (Game|SpawnActorfromClass "/Game/inkThrow/BP_inkExplosion.BP_inkExplosion_C" (Math|Transform|MakeTransform "0.000000,50000.000000,0.000000" "0, 0, 0" "1.000000,1.000000,1.000000") "Undefined" "MultiplyWithRoot" 0 0))
  (for _index (range 1 (Variables|Default|GetcandleLightPopulation))
    (bind _returnvalue_2 (Game|SpawnActorfromClass "/Game/ProcGen/Prototyping/bookInstanciating/otherBookshelfItems/BP_candle.BP_candle_C" (Variables|Default|GetfarAway) "AlwaysSpawn" "MultiplyWithRoot" 0 0))
    (Utilities|Array|Add (Variables|Default|GetcandleLightQueue) _returnvalue_2))
  (for _index_2 (range 1 (Variables|Default|GetinkBottlePopulation))
    (bind _returnvalue_3 (Game|SpawnActorfromClass "/Game/inkThrow/BP_inkItem.BP_inkItem_C" (Math|Transform|MakeTransform (.location _faraway) (.rotation _faraway) (Math|Conversions|ToVector(Float) (Math|Float|MakeLiteralFloat 1.0))) "AlwaysSpawn" "MultiplyWithRoot" 0 _returnvalue 0))
    (Utilities|Array|Add (Variables|Default|GetinkBottleQueue) _returnvalue_3)
    (Variables|/Game/inkThrow/BP_inkItem.BP_inkItem_C|SetparentQueue _returnvalue_3 self)))

(fn GetCamCompWorld
  (return "0, 0, 0"))

(fn TryPickup
  (params (item :type Actor%20Object%20Reference))
  (return false))

(fn TryThrow
  (params (direction :type Vector :default "0, 0, 0") (strength :type Float%20%28double-precision%29))
  (return false))