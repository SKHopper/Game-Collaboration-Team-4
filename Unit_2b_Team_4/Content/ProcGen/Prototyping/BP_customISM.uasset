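; Prototype instanced static mesh component for procedural generation that can look up instances by location.
; AddInstanceCustom records each instance's location in the LocationIndices array and writes X, Y and Z into per-instance custom data for material access.
; RemoveInstanceCustom deletes the instance and the array entry at the same index, keeping both lists parallel.
; FindInstanceIndex searches that array for an exact location to return its index.
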(fn AddInstanceCustom
  (params (InstanceTransform :type Transform%20%28by%20ref%29) (bWorldSpace :type Boolean))
  (bind _location (Math|Transform|BreakTransform InstanceTransform))
  (bind (_x _y _z) (Math|Vector|BreakVector _location))
  (bind _returnvalue (Components|InstancedStaticMesh|AddInstance InstanceTransform bWorldSpace))
  (Utilities|Array|Add (Variables|Default|GetlocationIndices) _location)
  (Components|InstancedStaticMesh|SetCustomDataValue _returnvalue 0 _x true)
  (Components|InstancedStaticMesh|SetCustomDataValue _returnvalue 1 _y true)
  (Components|InstancedStaticMesh|SetCustomDataValue _returnvalue 2 _z true)
  (return _returnvalue))

(fn RemoveInstanceCustom
  (params (InstanceIndex :type Integer))
  (if (Class|InstancedStaticMeshComponent|IsValidInstance InstanceIndex)
    (bind _returnvalue (Class|InstancedStaticMeshComponent|RemoveInstance InstanceIndex))
    (Utilities|Array|RemoveIndex (Variables|Default|GetlocationIndices) InstanceIndex)
    (return _returnvalue)))

(fn FindInstanceIndex
  (params (ItemToFind :type Vector%20%28by%20ref%29))
  (return (Utilities|Array|FindItem (Variables|Default|GetlocationIndices) ItemToFind)))