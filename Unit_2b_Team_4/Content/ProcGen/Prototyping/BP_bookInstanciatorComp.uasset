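; Book instancing component that procedurally fills bookshelves with books through a custom ISM wrapper.
; On BeginPlay it builds a grid of relative slot transforms from the case's shelf sections.
; A shelf's first generation randomly assigns each slot a book or a candle spot, caching book scales per bookshelf transform for later respawns.
; Spawned locations are stored per shelf so unloading can find and remove those instances.
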(event EventBeginPlay
  (CallFunction|LoadInstanceRelativeLocations))

(fn MakeBooksforShelf
  (params (firstGeneration :type Boolean) (bookshelfTransform :type Transform))
  (if firstGeneration
    (CallFunction|GenerateInstanceTransform bookshelfTransform))
  (CallFunction|InstanciateBooks bookshelfTransform))

(fn LoadInstanceRelativeLocations
  (for _array_element (Variables|Default|GetcaseShelfSections)
    (LocalVariables|SetcurrentSection _array_element)
    (for _index (range 0 (- (Variables|Default|GetitemsPerShelf) 1))
      (LocalVariables|Setlateral _index)
      (for _index_2 (range 0 (- (Variables|Default|GetshelvesPerCase) 1))
        (LocalVariables|Setvertical _index_2)
        (Utilities|Array|Add (Variables|Default|GetinstanceTransformsRelative) (Math|Transform|MakeTransform (+ (.location (LocalVariables|GetcurrentSection)) (Math|Vector|MakeVector 0.0 (* (+ (LocalVariables|Getlateral) -2) (Variables|Default|GetitemWidth)) (* (LocalVariables|Getvertical) (Variables|Default|GetshelfHeight)))) (.rotation (LocalVariables|GetcurrentSection)) "0.375000,0.375000,0.375000"))))))

(fn GenerateInstanceTransform
  (params (bookshelfTransform :type Transform%20%28by%20ref%29))
  (for (_ _array_index) (Variables|Default|GetinstanceTransformsRelative)
    (if (Math|Random|RandomBoolwithWeight (Variables|Default|GetweightBookSpawns))
      (Utilities|Array|SetArrayElem (LocalVariables|Getinstances) _array_index (Utilities|GenerateScale) true)
      (else
        (Default|GenerateCandleSpot (Variables|Default|GetcandleInstanciator) bookshelfTransform (Utilities|Array|Get(acopy) (Variables|Default|GetinstanceTransformsRelative) _array_index)))))
  (Utilities|Map|Add (Variables|Default|GetbookshelfInstances) bookshelfTransform (Utilities|Struct|MakeF_vectorArray (LocalVariables|Getinstances))))

(fn InstanciateBooks
  (params (bookshelfTransform :type Transform%20%28by%20ref%29))
  (bind _temp (LocalVariables|Gettemp))
  (for (_array_element _array_index) (.vectors (.Value (Utilities|Map|Find (Variables|Default|GetbookshelfInstances) bookshelfTransform)))
    (if (not (== (Math|Vector|VectorLength _array_element) 0.0))
      (bind _instanceworld (CallFunction|InstanciateBook (Math|Transform|MakeTransform (.Location (Math|Transform|BreakTransform (Utilities|Array|Get(acopy) (Variables|Default|GetinstanceTransformsRelative) _array_index))) (.Rotation (Math|Transform|BreakTransform (Utilities|Array|Get(acopy) (Variables|Default|GetinstanceTransformsRelative) _array_index))) (* (.Scale (Math|Transform|BreakTransform (Utilities|Array|Get(acopy) (Variables|Default|GetinstanceTransformsRelative) _array_index))) _array_element)) bookshelfTransform))
      (Utilities|Array|Add (LocalVariables|Gettemp) _instanceworld)))
  (Utilities|Map|Add (Variables|Default|GetloadedItems) (.location bookshelfTransform) (Utilities|Struct|MakeF_vectorArray _temp))
  (Variables|Default|Settest (+ (Variables|Default|Gettest) (Utilities|Array|Length _temp)))
  (Default|CheckInstanciate (Variables|Default|GetcandleInstanciator) bookshelfTransform))

(fn InstanciateBook
  (params (bookRelative :type Transform%20%28by%20ref%29) (bookshelfWorld :type Transform%20%28by%20ref%29))
  (bind _returnvalue (Math|Vector|RotateVector (.location bookRelative) (.rotation bookshelfWorld)))
  (bind _returnvalue_2 (+ _returnvalue (.location bookshelfWorld)))
  (Default|AddInstanceCustom (Variables|Default|GetcustomISM) (Math|Transform|MakeTransform _returnvalue_2 (Math|Rotator|CombineRotators (.rotation bookRelative) (.rotation bookshelfWorld)) (.scale bookRelative)) true)
  (return _returnvalue_2))

(fn UnloadBooksforShelf
  (params (bookshelfWorld :type Vector%20%28by%20ref%29))
  (bind _customism (Variables|Default|GetcustomISM))
  (for _array_element (.vectors (.Value (Utilities|Map|Find (Variables|Default|GetloadedItems) bookshelfWorld)))
    (bind _instanceindex (Default|FindInstanceIndex _customism _array_element))
    (Default|RemoveInstanceCustom _customism _instanceindex)))