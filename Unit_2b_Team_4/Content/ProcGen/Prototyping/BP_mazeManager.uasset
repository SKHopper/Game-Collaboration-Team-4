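; Procedural maze manager that streams an endless grid of walls and pillars around the player pawn.
; Each tick it snaps the player to a grid point, queues missing nearby points to load and points beyond the cull distance to unload.
; New points roll four weighted random wall sides, saved in a map so revisits rebuild identically.
; Meshes are custom ISM instances, removed by matching their XY locations against the unload queue.
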(event EventBeginPlay
  (Variables|Default|Setplayer (Game|Player|GetPlayerPawn 0)))

(event EventTick
  (params (DeltaSeconds :type Float%20%28single-precision%29))
  (Variables|Default|SetclosestPlayerPoint (Utilities|FindClosestPlayerPoint))
  (bind _queue (CallFunction|QueuePointstoLoad))
  (CallFunction|InstanciateMeshes _queue)
  (bind _queue_2 (CallFunction|QueuePointstoUnload))
  (CallFunction|UninstanciateMeshes _queue_2))

(fn ConstructionScript
  (CallFunction|SetupCullDistance))

(fn GetGridRelativePoints
  (for _index (range 0 (Variables|Default|GetgridLoadWidth))
    (LocalVariables|Setx _index)
    (for _index_2 (range 0 (Variables|Default|GetgridLoadWidth))
      (LocalVariables|Sety _index_2)
      (Utilities|Array|Add (LocalVariables|GetoutLocations) (Utilities|GetGridPointLocation (LocalVariables|Getx) (LocalVariables|Gety)))))
  (return (LocalVariables|GetoutLocations)))

(fn InstanciateMeshes
  (params (queue :type Array%20of%20Vector%202D%20Structures))
  (for _array_element queue
    (Utilities|Array|Add (Variables|Default|GetloadedPoints) _array_element)
    (CallFunction|InstanciatePointWalls (Math|Vector|MakeVector (.X (Math|Vector2D|BreakVector2D _array_element)) (.Y (Math|Vector2D|BreakVector2D _array_element)) 0.0) _array_element)))

(fn InstanciatePointWalls
  (params (location :type Vector) (location2D :type Vector%202D%20Structure))
  (bind _output_get (LocalVariables|SetalreadySaved (Utilities|Map|Contains (Variables|Default|GetsavedPoints) location2D)))
  (if _output_get
    (for (_array_element _array_index) (.sides (.Value (Utilities|Map|Find (Variables|Default|GetsavedPoints) location2D)))
      (if _array_element
        (LocalVariables|SetsideIndex _array_index)
        (LocalVariables|SetneedsPillar true)
        (CallFunction|InstanceSide (Math|Vector|MakeVector (.x location2D) (.y location2D) 0.0) (LocalVariables|GetsideIndex) (LocalVariables|GetsideIndex))))
    (else
      (Utilities|Map|Add :TargetMap (Variables|Default|GetsavedPoints) :Key location2D)
      (for _index (range 0 3)
        (LocalVariables|SetsideIndex _index)
        (if (Math|Random|RandomBoolwithWeight (Variables|Default|GetweightWallSpawns))
          (CallFunction|SaveSide location2D (LocalVariables|GetsideIndex))
          (LocalVariables|SetneedsPillar true)
          (CallFunction|InstanceSide (Math|Vector|MakeVector (.x location2D) (.y location2D) 0.0) (LocalVariables|GetsideIndex) (LocalVariables|GetsideIndex))))
      (if (LocalVariables|GetneedsPillar)
        (CallFunction|InstancePillar location)))))

(fn QueuePointstoLoad
  (bind _gridloadwidth (Variables|Default|GetgridLoadWidth))
  (bind _returnvalue (/ _gridloadwidth 2))
  (bind _returnvalue_2 (- _returnvalue _gridloadwidth))
  (for _index (range _returnvalue_2 _returnvalue)
    (bind _output_get (LocalVariables|Setx _index))
    (for _index_2 (range _returnvalue_2 _returnvalue)
      (bind _output_get_2 (LocalVariables|Sety _index_2))
      (if (not (Utilities|Array|ContainsItem (Variables|Default|GetloadedPoints) (Utilities|GetPlayerRelativePointWorld _output_get _output_get_2)))
        (Utilities|Array|Add (LocalVariables|GetoutQueue) (Utilities|GetPlayerRelativePointWorld _output_get _output_get_2)))))
  (return (LocalVariables|GetoutQueue)))

(fn QueuePointstoUnload
  (for _array_element (Variables|Default|GetloadedPoints)
    (if (Utilities|IsPointFarAway _array_element)
      (Utilities|Array|Add (LocalVariables|GetoutQueue) _array_element)
      (for (_array_element_2 _array_index) (.sides (.Value (Utilities|Map|Find (Variables|Default|GetsavedPoints) _array_element)))
        (if _array_element_2
          (Utilities|Array|Add (LocalVariables|GetoutQueue) (+ _array_element (Math|Vector2D|MakeVector2D (.x (Utilities|GetWallOffset _array_index (Utilities|SideLength))) (.y (Utilities|GetWallOffset _array_index (Utilities|SideLength))))))))))
  (return (LocalVariables|GetoutQueue)))

(fn InstancePillar
  (params (Instance%20Transform%20Location :type Vector))
  (bind _meshwidthmultiplier (Variables|Default|GetmeshWidthMultiplier))
  (Default|AddInstanceCustom (Variables|Default|GetcustomISM) (Math|Transform|MakeTransform Instance%20Transform%20Location "0, 0, 0" (Math|Vector|MakeVector _meshwidthmultiplier _meshwidthmultiplier (Variables|Default|GetwallHeight))) false))

(fn InstanceSide
  (params (A :type Vector) (A2 :type Integer) (directionIndex :type Integer))
  (bind _returnvalue (Utilities|SideLength))
  (bind _returnvalue_2 (Default|AddInstanceCustom (Variables|Default|GetcustomISM) (Math|Transform|MakeTransform (+ A (Utilities|GetWallOffset directionIndex _returnvalue)) (Math|Rotator|MakeRotator 0.0 0.0 (Math|Conversions|ToFloat(Integer) (* A2 90))) (Math|Vector|MakeVector (/ _returnvalue (Variables|Default|GetmeshWidth)) (Variables|Default|GetmeshWidthMultiplier) (Variables|Default|GetwallHeight))) false)))

(fn SaveSide
  (params (Key :type Vector%202D%20Structure%20%28by%20ref%29) (Index :type Integer))
  (bind _savedpoints (Variables|Default|GetsavedPoints))
  (bind _output_get (LocalVariables|Settemp (.sides (.Value (Utilities|Map|Find _savedpoints Key)))))
  (Utilities|Array|SetArrayElem _output_get Index true)
  (Utilities|Map|Add _savedpoints Key (Utilities|Struct|MakeF_gridPointSides _output_get)))

(fn SetupCullDistance
  (Variables|Default|SetcullDistance (* (/ (* (Math|Conversions|ToFloat(Integer) (Variables|Default|GetgridLoadWidth)) (Variables|Default|GetcullWidthScale)) 2.0) (Variables|Default|GetgridSectionWidth))))

(fn UninstanciateMeshes
  (params (queue :type Array%20of%20Vector%202D%20Structures))
  (for _index (range 0 (- (Components|InstancedStaticMesh|GetInstanceCount) 1))
    (if (Utilities|Array|ContainsItem queue (Math|Vector2D|MakeVector2D (.x (.location (.OutInstanceTransform (Components|InstancedStaticMesh|GetInstanceTransform (Variables|Default|GetcustomISM) _index false)))) (.y (.location (.OutInstanceTransform (Components|InstancedStaticMesh|GetInstanceTransform (Variables|Default|GetcustomISM) _index false))))))
      (Default|RemoveInstanceCustom (Variables|Default|GetcustomISM) _index)
      (Utilities|Array|RemoveItem (Variables|Default|GetloadedPoints) (Math|Vector2D|MakeVector2D (.x (.location (.OutInstanceTransform (Components|InstancedStaticMesh|GetInstanceTransform (Variables|Default|GetcustomISM) _index false)))) (.y (.location (.OutInstanceTransform (Components|InstancedStaticMesh|GetInstanceTransform (Variables|Default|GetcustomISM) _index false)))))))))

(fn SlowContains
  (params (TargetArray :type Array%20of%20Vector%202D%20Structures) (ItemToFind :type Vector%202D%20Structure%20%28by%20ref%29))
  (for _array_element TargetArray
    (if (Utilities|Operators|EqualEqual ItemToFind _array_element 1e+03)
      (return true)))
  (return false))