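; Prototype navigation-map component for a procedurally generated maze, recording which grid points are closed off in a map keyed by integer XY.
; AddPointsAround writes 3x3 blocks around a centre point, and queries treat ungenerated points as blocked.
; World/grid conversions use the owning maze manager's section size divided by three, relative to the owner's location.
; A test event draws the map as debug circles; older four-quadrant array storage remains as unreachable code.
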(event EventBeginPlay
  (CallFunction|ContactParent))

(fn AddPointsAround
  (params (centrePoint :type Int%20Vector%202%20Structure) (points :type Array%20of%20F%20Boolean%20Array%20Structures))
  (bind (_x _y) (Utilities|Struct|BreakIntVector2 centrePoint))
  (bind _xy (LocalVariables|Getxy))
  (for _index (range -1 1)
    (Utilities|Struct|SetmembersinIntVector2 _xy (+ _index _x))
    (for _index_2 (range -1 1)
      (bind _structout (Utilities|Struct|SetmembersinIntVector2 _xy (+ _y _index_2)))
      (CallFunction|SetMapValue _structout (Utilities|Array|Get(acopy) (.booleans (Utilities|Array|Get(acopy) points (+ _index 1))) (+ _index_2 1))))))

(fn SetMapValue
  (params (xy :type Int%20Vector%202%20Structure) (closedOff :type Boolean))
  (Utilities|Map|Add (Variables|Default|GetmapSet) (Utilities|Struct|MakeIntVector2 (.x xy) (.y xy)) closedOff))

(fn UpdateMapXSize
  (params (mapQuadrant :type Integer) (x :type Integer))
  (bind _returnvalue (- x 1))
  (if (not (> (Utilities|Select :Index mapQuadrant :Option%200 (Utilities|Array|Length (Variables|Default|Getmap)) :Option%201 (Utilities|Array|Length (Variables|Default|GetmapNegX)) :Option%202 (Utilities|Array|Length (Variables|Default|GetmapNegY)) :Option%203 (Utilities|Array|Length (Variables|Default|GetmapNegXY))) x))
    (switch int mapQuadrant
      (:0
        (Utilities|Array|SetArrayElem :TargetArray (Variables|Default|Getmap) :Index x :bSizeToFit true))
      (:1
        (Utilities|Array|SetArrayElem :TargetArray (Variables|Default|GetmapNegX) :Index _returnvalue :bSizeToFit true))
      (:2
        (Utilities|Array|SetArrayElem :TargetArray (Variables|Default|GetmapNegY) :Index x :bSizeToFit true))
      (:3
        (Utilities|Array|SetArrayElem :TargetArray (Variables|Default|GetmapNegXY) :Index _returnvalue :bSizeToFit true)))))

(fn GetQuadrant
  (params (xy :type Int%20Vector%202%20Structure%20%28by%20ref%29))
  (bind (_x _y) (Utilities|Struct|BreakIntVector2 xy))
  (bind _returnvalue (> _y -1))
  (if (> _x -1)
    (if _returnvalue
      (return 0)
      (else
        (return 2)))
    (elif _returnvalue
      (return 1)
      (else
        (return 3)))))

(fn ContactParent
  (bind _asif_maze_manager (Utilities|Casting|CastToIF_mazeManager (Components|GetOwner)))
  (Variables|Default|SetparentManager _asif_maze_manager))

(event Custom|test
  (bind (_keypin _valuepin) (Utilities|Map|ForEachLoop(Map) (Variables|Default|GetmapSet))
    (:then
      (Rendering|Debug|DrawDebugCircle (Math|Vector|MakeVector (.x (/ (* (Math|Vector|MakeVector (Math|Conversions|ToFloat(Integer) (.x _keypin)) (Math|Conversions|ToFloat(Integer) (.y _keypin)) 0.0) 1e+03) 3.0)) (.y (/ (* (Math|Vector|MakeVector (Math|Conversions|ToFloat(Integer) (.x _keypin)) (Math|Conversions|ToFloat(Integer) (.y _keypin)) 0.0) 1e+03) 3.0)) 3e+02) 3e+01 12 (Math|Color|SelectColor "(R=1.000000,G=0.000000,B=0.000000,A=1.000000)" "(R=0.000000,G=1.000000,B=0.000000,A=1.000000)" _valuepin) 2e+01 2e+01 "0.000000,1.000000,0.000000" "0.000000,0.000000,1.000000"))))

(fn GetIsPointBlocked
  (params (point :type Int%20Vector%202%20Structure))
  (bind _mapset (Variables|Default|GetmapSet))
  (bind (_value _returnvalue) (Utilities|Map|Find _mapset point))
  (return (or _value (not _returnvalue)) _returnvalue))

(fn NavGridtoWorld
  (params (in :type Int%20Vector%202%20Structure))
  (bind _returnvalue (Components|GetOwner))
  (bind _returnvalue_2 (Transformation|GetActorLocation _returnvalue))
  (bind _size (Default|GetLargeGridSectionSide (Variables|Default|GetparentManager)))
  (return (+ (* (Math|Vector2D|MakeVector2D (Math|Conversions|ToFloat(Integer) (.x in)) (Math|Conversions|ToFloat(Integer) (.y in))) (Math|Vector2D|MakeVector2D (/ _size 3.0) (/ _size 3.0))) (Math|Vector2D|MakeVector2D (.x _returnvalue_2) (.y _returnvalue_2)))))

(fn WorldtoNavGrid
  (params (in :type Vector%202D%20Structure))
  (bind _returnvalue (Components|GetOwner))
  (bind _returnvalue_2 (Transformation|GetActorLocation _returnvalue))
  (bind _size (Default|GetLargeGridSectionSide (Variables|Default|GetparentManager)))
  (return (Utilities|Struct|MakeIntVector2 (Math|Float|Round (.x (/ (- (Math|Vector2D|MakeVector2D (.x in) (.y in)) (Math|Vector2D|MakeVector2D (.x _returnvalue_2) (.y _returnvalue_2))) (/ _size 3.0)))) (Math|Float|Round (.y (/ (- (Math|Vector2D|MakeVector2D (.x in) (.y in)) (Math|Vector2D|MakeVector2D (.x _returnvalue_2) (.y _returnvalue_2))) (/ _size 3.0)))))))