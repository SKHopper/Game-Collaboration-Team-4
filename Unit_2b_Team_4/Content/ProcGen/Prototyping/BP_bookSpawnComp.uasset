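; Maze manager component that spawns a new book whenever one is picked up and reports it to the compass.
; NewBook retries random large-grid cells within a spawn radius until one is far enough from the player.
; Generated cells without occupied sides are rerolled, while ungenerated cells get the book directly.
; In generated cells, the book moves after a short delay to a random free-spot transform on that side's bookshelf.
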(event Custom|adjustBookToSpot
  (params (side :type Integer))
  (bind _lastbookspawnworld (Variables|Default|GetlastBookSpawnWorld))
  (Utilities|FlowControl|Delay 0.5)
  (bind _transformout (Default|FindBookshelf (Variables|Default|Getparent) (Math|Vector|MakeVector (.x _lastbookspawnworld) (.y _lastbookspawnworld) 0.0) side))
  (Development|PrintString (Utilities|String|ToString(Vector) (.location (.OutItem (Utilities|Array|Random (.transforms (.Value (Utilities|Map|Find (Variables|/Game/ProcGen/Prototyping/bookInstanciating/otherBookshelfItems/BP_candleComp.BP_candleComp_C|GetfreeSpots (Variables|Default|GetfreeSpotsCandleComp)) _transformout))))))))
  (Transformation|SetActorTransform (Variables|Default|GetlastBook) (Math|Transform|MakeTransform (+ (.Location (Math|Transform|BreakTransform _transformout)) (Math|Vector|RotateVector (.location (.OutItem (Utilities|Array|Random (.transforms (.Value (Utilities|Map|Find (Variables|/Game/ProcGen/Prototyping/bookInstanciating/otherBookshelfItems/BP_candleComp.BP_candleComp_C|GetfreeSpots (Variables|Default|GetfreeSpotsCandleComp)) _transformout)))))) (.Rotation (Math|Transform|BreakTransform _transformout)))) (Math|Rotator|CombineRotators (.Rotation (Math|Transform|BreakTransform _transformout)) (.rotation (.OutItem (Utilities|Array|Random (.transforms (.Value (Utilities|Map|Find (Variables|/Game/ProcGen/Prototyping/bookInstanciating/otherBookshelfItems/BP_candleComp.BP_candleComp_C|GetfreeSpots (Variables|Default|GetfreeSpotsCandleComp)) _transformout))))))) "1.000000,1.000000,1.000000")))

(event EventBeginPlay
  (bind _asbp_maze_manager (Utilities|Casting|CastToBP_mazeManager (Components|GetOwner)))
  (Variables|Default|Setparent _asbp_maze_manager))

(event EventReportBookPickedUp
  (CallFunction|NewBook))

(event EventReportCompass
  (params (compass :type IF%20Compass%20Maze%20Interface))
  (Variables|Default|Setcompass compass))

(fn NewBook
  (bind _largegrid (Default|GetWorldtoLargeGrid (Variables|Default|Getparent) (Math|Conversions|ToVector2D(Vector) (LocalVariables|GetbookSpawnPlayerMinDistance))))
  (LocalVariables|SetgridPlayerMinDistance (.x _largegrid))
  (Utilities|FlowControl|ForLoopwithBreak 0 555 :!label _label
    (:LoopBody
      (bind (_grid_distance _location) (Utilities|TryFindBookLargeGrid))
      (bind _output_get (LocalVariables|SetdistanceToPlayer _grid_distance))
      (LocalVariables|SetspawnGridLocation _location)
      (if (not (< _output_get (LocalVariables|GetgridPlayerMinDistance)))
        (goto _label Break)))
    (:Completed
      (bind _world (Default|GetLargeGridtoWorld (Variables|Default|Getparent) (LocalVariables|GetspawnGridLocation)))
      (bind _output_get_2 (Variables|Default|SetlastBookSpawnWorld _world))
      (bind (_generated _side _empty) (CallFunction|LastBookGeneration))
      (if _generated
        (if _empty
          (goto _label)
          (else
            (CallFunction|SpawnBook (.x _output_get_2) (.y _output_get_2))
            (CallFunction|AdjustBooktoSpot _side)))
        (else
          (CallFunction|SpawnBook (.x _output_get_2) (.y _output_get_2)))))))

(fn SpawnBook
  (params (Spawn%20Transform%20Location%20X :type Float%20%28double-precision%29) (Spawn%20Transform%20Location%20Y :type Float%20%28double-precision%29))
  (bind _returnvalue (Game|SpawnActorfromClass "/Game/memoryBook/testBook.testBook_C" (Math|Transform|MakeTransform (Math|Vector|MakeVector Spawn%20Transform%20Location%20X Spawn%20Transform%20Location%20Y 0.0) "0, 0, 0" "1.000000,1.000000,1.000000") "Undefined" "MultiplyWithRoot" 0 0))
  (bind _output_get (Variables|Default|SetlastBook _returnvalue))
  (Variables|/Game/memoryBook/testBook.testBook_C|SetparentSpawner _output_get self)
  (Default|ReportNewBook (Variables|Default|Getcompass) (Variables|Default|GetlastBook)))

(fn LastBookGeneration
  (bind _parent (Variables|Default|Getparent))
  (bind _lastbookspawnworld (Variables|Default|GetlastBookSpawnWorld))
  (bind _savedpoints (Variables|/Game/ProcGen/Prototyping/BP_mazeManager.BP_mazeManager_C|GetsavedPoints _parent))
  (bind (_value _returnvalue) (Utilities|Map|Find _savedpoints _lastbookspawnworld))
  (if _returnvalue
    (for (_array_element _array_index) (.sides _value)
      (if _array_element
        (return true _array_index false)))
    (return true 0 true)
    (else
      (return false 0 false))))