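; Player marker painter for the procedural map, rendering a single brush stamp into a render target.
; SetupDrawing creates the render target, a display material that samples it as "player", and a brush material using the UE logo texture, then returns the display material.
; The draw event clears the target each call and draws the brush centered on a normalized location, sized by BrushSize and a multiplier, so no trail accumulates.
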(event Custom|draw
  (params (location :type Vector%202D%20Structure) (brushMult :type Float%20%28double-precision%29))
  (bind _returnvalue (Math|Float|MakeLiteralFloat 1024.0))
  (bind _brushsize (Variables|Default|GetbrushSize))
  (bind _returnvalue_2 (* brushMult _returnvalue))
  (bind _returnvalue_3 (* _returnvalue_2 _brushsize))
  (Rendering|ClearRenderTarget2D (Variables|Default|GetrenderTarget))
  (bind (_canvas _size _context) (Rendering|BeginDrawCanvastoRenderTarget (Variables|Default|GetrenderTarget)))
  (Canvas|DrawMaterial :self _canvas :RenderMaterial (Variables|Default|Getbrush) :ScreenPosition (- (* _size location) (/ _returnvalue_3 2.0)) :ScreenSize (Math|Vector2D|MakeVector2D _returnvalue_3 _returnvalue_3) :CoordinateSize "(X=1.000000,Y=1.000000)" :PivotPoint "(X=0.500000,Y=0.500000)")
  (Rendering|EndDrawCanvastoRenderTarget _context))

(fn SetupDrawing
  (bind _returnvalue (Rendering|CreateRenderTarget2D 1024 1024 "RTF_RGBA16f"))
  (bind _output_get (Variables|Default|SetrenderTarget _returnvalue))
  (Rendering|ClearRenderTarget2D _output_get)
  (bind _returnvalue_2 (Rendering|Material|CreateDynamicMaterialInstance "/Game/ProcGen/map/playerMarker/M_playerMarker.M_playerMarker" "None" "None" :!class /Script/Engine.KismetMaterialLibrary))
  (bind _output_get_2 (Variables|Default|Setcanvas _returnvalue_2))
  (Rendering|Material|SetTextureParameterValue _output_get_2 "player" (Variables|Default|GetrenderTarget))
  (bind _returnvalue_3 (Rendering|Material|CreateDynamicMaterialInstance "/Game/ProcGen/map/M_testDrawBrush.M_testDrawBrush" "None" "None" :!class /Script/Engine.KismetMaterialLibrary))
  (bind _output_get_3 (Variables|Default|Setbrush _returnvalue_3))
  (Rendering|Material|SetTextureParameterValue _output_get_3 "brushTexture" "/Game/Characters/Mannequins/Textures/Shared/T_UE_Logo_M.T_UE_Logo_M")
  (return _output_get_2))