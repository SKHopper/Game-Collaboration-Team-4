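; Map component that spawns a BP_map actor and shows its nav-map drawing in the player's inventory map widget.
; Setup registers with all IF_map actors and hands the map's canvas material and player to the widget.
; Activation reveals the map, saves a flag to the GameInstance and redraws; generation reports redraw it while active.
; BeginPlay activates immediately if that flag is set, and unconditionally after a one-second delay.
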(event EventBeginPlay
  (CallFunction|Setup)
  (bind _hasmap (Class|IFSave|GetHasMap(Message) (Game|GetGameInstance)))
  (if _hasmap
    (CallFunction|ActivateMap))
  (Utilities|FlowControl|Delay 1.0)
  (CallFunction|ActivateMap)
  (if (Variables|Default|Getactive)
    (CallFunction|Update)))

(event EventActivateMap
  (Default|SetMapVisibility (Variables|Default|Getinventory) true)
  (Class|IFSave|SetHasMap(Message) (Game|GetGameInstance) true)
  (Variables|Default|Setactive true)
  (CallFunction|Update))

(event EventReportGenUpdate
  (if (Variables|Default|Getactive)
    (CallFunction|Update)))

(fn Setup
  (bind _returnvalue (Game|Player|GetPlayerPawn 0))
  (bind _returnvalue_2 (Actor|GetComponentbyClass _returnvalue "/Game/Inventory/BP_inventoryComp.BP_inventoryComp_C"))
  (bind _inventorywidget (Variables|/Game/Inventory/BP_inventoryComp.BP_inventoryComp_C|GetinventoryWidget _returnvalue_2))
  (bind _outactors (Actor|GetAllActorswithInterface "/Game/ProcGen/map/IF_map.IF_map_C"))
  (for _array_element _outactors
    (Class|IFMap|ReportSelf(Message) _array_element self))
  (bind _returnvalue_3 (Game|SpawnActorfromClass "/Game/ProcGen/map/BP_map.BP_map_C" (Math|Transform|MakeTransform "0, 0, 0" "0, 0, 0" "1.000000,1.000000,1.000000") "Undefined" "MultiplyWithRoot" 0 0))
  (bind _output_get (Variables|Default|Setmap _returnvalue_3))
  (bind (_canvas _player) (Default|Setup _output_get))
  (Variables|Default|Setinventory _inventorywidget)
  (bind _output_get_2 (Variables|Default|Setwidget (Variables|/Game/Inventory/WBP_inventory.WBP_inventory_C|GetWBP_map _inventorywidget)))
  (Default|SetMap _output_get_2 _canvas _player))

(fn Update
  (Default|DrawNavMap (Variables|Default|Getmap)))