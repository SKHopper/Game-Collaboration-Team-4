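; Map spawner that scatters map item pickups around the world at BeginPlay for the player to find.
; SpawnItems places SpawnCount BP_mapItem actors at random yaw and distance (1000 to SpawnRadius) around the world origin, storing each and setting itself as Parent.
; PickedUp destroys every stored item, calling ActivateMapMessage on the player pawn once per item inside the loop.
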(event EventBeginPlay
  (CallFunction|SpawnItems))

(fn SpawnItems
  (bind _returnvalue (Math|Random|RandomFloatinRange 0.0 359.0))
  (bind _returnvalue_2 (Math|Rotator|MakeRotator 0.0 0.0 _returnvalue))
  (for _index (range 0 (- (Variables|Default|GetspawnCount) 1))
    (bind _returnvalue_3 (Game|SpawnActorfromClass "/Game/ProcGen/map/BP_mapItem.BP_mapItem_C" (Math|Transform|MakeTransform (Math|Vector|RotateVector (Math|Vector|MakeVector (Math|Random|RandomFloatinRange 1e+03 (Variables|Default|GetspawnRadius)) 0.0 0.0) _returnvalue_2) _returnvalue_2 "1.000000,1.000000,1.000000") "Undefined" "MultiplyWithRoot" 0 0))
    (Utilities|Array|Add (Variables|Default|GetmapItems) _returnvalue_3)
    (Variables|/Game/ProcGen/map/BP_mapItem.BP_mapItem_C|Setparent _returnvalue_3 self)))

(fn PickedUp
  (for _array_element (Variables|Default|GetmapItems)
    (Actor|DestroyActor _array_element)
    (Class|IFInventory|ActivateMap(Message) (Game|Player|GetPlayerPawn 0))))