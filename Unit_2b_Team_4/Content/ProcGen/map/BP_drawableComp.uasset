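; Component in the procedural generation map folder that paints brush stamps at given locations onto a runtime render target.
; On BeginPlay it creates and clears the render target, then builds dynamic materials: a canvas that samples the target and a brush carrying the brush texture.
; The draw event clears the target and stamps the brush centered on each location, treating locations as normalized canvas coordinates, so each call replaces the previous drawing.
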(event Custom|draw
  (params (location :type Array%20of%20Vector%202D%20Structures))
  (bind _brushsize (Variables|Default|GetbrushSize))
  (Rendering|ClearRenderTarget2D (Variables|Default|GetrenderTarget))
  (bind (_canvas _size _context) (Rendering|BeginDrawCanvastoRenderTarget (Variables|Default|GetrenderTarget)))
  (for _array_element location
    (Canvas|DrawMaterial :self _canvas :RenderMaterial (Variables|Default|Getbrush) :ScreenPosition (- (* _size _array_element) (/ (Variables|Default|GetbrushSize) 2.0)) :ScreenSize (Math|Vector2D|MakeVector2D _brushsize _brushsize) :CoordinateSize "(X=1.000000,Y=1.000000)" :PivotPoint "(X=0.500000,Y=0.500000)"))
  (Rendering|EndDrawCanvastoRenderTarget _context))

(event EventBeginPlay
  (CallFunction|SetupDrawing))

(fn SetupDrawing
  (bind _returnvalue (Rendering|CreateRenderTarget2D 1024 1024 "RTF_RGBA16f"))
  (bind _output_get (Variables|Default|SetrenderTarget _returnvalue))
  (Rendering|ClearRenderTarget2D _output_get)
  (bind _returnvalue_2 (Rendering|Material|CreateDynamicMaterialInstance (Variables|Default|GetcanvasParentInterface) "None" "None" :!class /Script/Engine.KismetMaterialLibrary))
  (bind _output_get_2 (Variables|Default|Setcanvas _returnvalue_2))
  (Rendering|Material|SetTextureParameterValue _output_get_2 "renderTarget" (Variables|Default|GetrenderTarget))
  (bind _returnvalue_3 (Rendering|Material|CreateDynamicMaterialInstance (Variables|Default|GetbrushParentInterface) "None" "None" :!class /Script/Engine.KismetMaterialLibrary))
  (bind _output_get_3 (Variables|Default|Setbrush _returnvalue_3))
  (Rendering|Material|SetTextureParameterValue _output_get_3 "brushTexture" (Variables|Default|GetbrushTexture)))