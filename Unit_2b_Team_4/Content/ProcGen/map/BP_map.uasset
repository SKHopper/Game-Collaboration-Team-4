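; BP_map draws a map of the procedurally generated maze, plus a marker for the player's position.
; On BeginPlay it gets the level width and nav component from the maze manager interface, sets up both drawing components, and starts a looping player-marker timer.
; DrawNavMap, not called here, draws the nav component's new-generation cells.
; Grid positions are normalized to map extents, with brush size scaled to match.
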(event Custom|drawPlayerMarker
  (bind _out (Default|WorldtoNavGrid (Variables|Default|GetnavComp) (Math|Conversions|ToVector2D(Vector) (Transformation|GetActorLocation (Game|Player|GetPlayerPawn 0)))))
  (Default|Draw (Variables|Default|GetplayerMarker) (Utilities|Normalize _out (Variables|Default|GetnavExtents) (Variables|Default|GetnavNormalization)) (Variables|Default|GetbrushMult)))

(event EventBeginPlay
  (CallFunction|Setup)
  (Utilities|Time|SetTimerbyEvent (delegate Custom|drawPlayerMarker) 0.2 true true))

(fn ConstructionScript)

(fn DrawNavMap
  (bind _levelwidth (Variables|Default|GetlevelWidth))
  (bind _returnvalue (Math|Float|Truncate _levelwidth))
  (bind _returnvalue_2 (Math|Conversions|ToFloat(Integer) _returnvalue))
  (Utilities|Set|Clear (Variables|Default|GetdrawLocations))
  (bind _output_get (Variables|Default|SetnavNormalization (Math|Vector2D|MakeVector2D _returnvalue_2 _returnvalue_2)))
  (bind _output_get_2 (Variables|Default|SetnavExtents (Math|Vector2D|MakeVector2D (+ (.x _output_get) _levelwidth) (+ (.y _output_get) _levelwidth))))
  (bind _wholegrid (Default|GetNewGeneration (Variables|Default|GetnavComp)))
  (bind _valuepin (Utilities|Set|ForEachLoop(Set) _wholegrid)
    (:then
      (Utilities|Set|Add (Variables|Default|GetdrawLocations) (Utilities|Normalize _valuepin _output_get_2 (Variables|Default|GetnavNormalization))))
    (:CompletedPin
      (bind _output_get_3 (Variables|Default|SetbrushMult (/ 1.0 (Math|Float|Max(Float) (.X (Math|Vector2D|BreakVector2D _output_get_2)) (.Y (Math|Vector2D|BreakVector2D _output_get_2))))))
      (Default|Draw (Variables|Default|Getdrawable) (Variables|Default|GetdrawLocations) _output_get_3))))

(fn Setup
  (bind _outactors (Actor|GetAllActorswithInterface "/Game/ProcGen/Prototyping/IF_mazeManager.IF_mazeManager_C"))
  (bind _width (Class|IFMazeManager|GetLevelWidth(Message) (Utilities|Array|Get(acopy) _outactors)))
  (Variables|Default|SetlevelWidth _width)
  (bind _mapcomp (Class|IFMazeManager|GetMapComp(Message) (Utilities|Array|Get(acopy) _outactors)))
  (Variables|Default|SetnavComp _mapcomp)
  (bind _canvas (Default|SetupDrawing (Variables|Default|Getdrawable)))
  (bind _output_get (Default|SetupDrawing (Variables|Default|GetplayerMarker)))
  (return _canvas _output_get))