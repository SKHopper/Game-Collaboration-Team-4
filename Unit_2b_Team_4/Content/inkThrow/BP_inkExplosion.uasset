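; BP_inkExplosion is a relocatable actor that plays the shattering of a thrown ink bottle at a given location.
; Explode plays an attenuated impact sound, teleports the actor there, resets and reveals the bottle Geometry Collection with physics on, and spawns a Niagara effect.
; It then calls Unexplode, which applies a radial impulse next tick, then hides the pieces and stops simulation after a short delay, leaving the actor reusable.
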(event Custom|unexplode
  (bind _gc_bottle (Variables|Default|GetGC_bottle))
  (bind _gc_bottle_2 (Variables|Default|GetGC_bottle))
  (Utilities|FlowControl|DelayUntilNextTick)
  (Physics|AddRadialImpulse _gc_bottle_2 (- (Transformation|GetWorldLocation _gc_bottle_2) "0.000000,0.000000,10.000000") 1e+03 5e+02 "RIF_Constant" true)
  (Utilities|FlowControl|Delay 2.0)
  (Rendering|SetVisibility _gc_bottle false false)
  (Physics|SetSimulatePhysics _gc_bottle false))

(fn ConstructionScript)

(fn Explode
  (params (NewLocation :type Vector) (VolumeMultiplier :type Float%20%28single-precision%29))
  (bind _gc_bottle (Variables|Default|GetGC_bottle))
  (Audio|PlaySoundatLocation "/Game/ASSET/audio/sfx_pack/ink_bottle_impact.ink_bottle_impact" NewLocation "0, 0, 0" VolumeMultiplier 1.0 0.0 "/Game/SOUND/SA_ink.SA_ink" 0 0 0)
  (Transformation|SetActorLocation NewLocation false true)
  (Rendering|SetVisibility _gc_bottle true false)
  (Class|GeometryCollectionComponent|SetRestCollection _gc_bottle "/Game/inkThrow/GC_bottle.GC_bottle" true)
  (Physics|SetSimulatePhysics _gc_bottle true)
  (Niagara|SpawnSystematLocation "/Game/MatsFolder/Niagara/NS_Throwable.NS_Throwable" NewLocation)
  (CallFunction|Unexplode))