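; BP_inkItem is a throwable ink item that the player can pick up and that makes noise on impact.
; TryInteract sends the player pawn a pickup message, and TryThrow enables physics on the Cube, applies a velocity impulse and marks it active.
; A valid overlap deactivates it, emits noise, stops physics and reports to ParentQueue.
; ValidCollision's player-exclusion and Active check is left unconnected.
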(event OnComponentBeginOverlap(Cube)
  (params (OverlappedComponent :type Primitive%20Component%20Object%20Reference) (OtherActor :type Actor%20Object%20Reference) (OtherComp :type Primitive%20Component%20Object%20Reference) (OtherBodyIndex :type Integer) (bFromSweep :type Boolean) (SweepResult :type Hit%20Result%20Structure%20%28by%20ref%29))
  (if (Utilities|ValidCollision OtherActor)
    (Variables|Default|Setactive false)
    (Default|Emitt (Variables|Default|GetnoiseEmitter) (Variables|Default|GetnoiseRadius) true "0, 0, 0" "ForDuration")
    (Physics|SetSimulatePhysics (Variables|Default|GetCube) false)
    (Default|ReportThrown (Variables|Default|GetparentQueue) self)))

(fn ConstructionScript)

(fn GetCamCompWorld
  (return "0, 0, 0"))

(fn TryInteract
  (Class|IFInk|TryPickup(Message) (Game|Player|GetPlayerPawn 0) self)
  (return false))

(fn TryThrow
  (params (direction :type Vector :default "0, 0, 0") (strength :type Float%20%28double-precision%29))
  (bind _cube (Variables|Default|GetCube))
  (Physics|SetSimulatePhysics _cube true)
  (Physics|AddImpulse _cube (* direction strength) "None" true)
  (Variables|Default|Setactive true)
  (return false))