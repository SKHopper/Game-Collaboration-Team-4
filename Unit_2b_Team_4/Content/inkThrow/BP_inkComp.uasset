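; Scene component for the ink-throw mechanic that holds a picked-up item, then throws or consumes it.
; When unlocked, pickup snaps the item to the component and shows an ink indicator widget.
; Throws message the item with its own ThrowStrength, aiming from the player's camera through a point just above the component, ignoring passed-in direction and strength.
; Consuming messages the item and adds ink to the Companion.
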(event EventBeginPlay
  (bind _returnvalue (UserInterface|CreateWidget "/Game/indicatorUI/WBP_inkIndicator.WBP_inkIndicator_C"))
  (Variables|Default|Setindicator _returnvalue))

(fn PrepforThrow
  (params (item :type Actor%20Object%20Reference))
  (bind _output_get (Variables|Default|SetlastHeldItem item))
  (Transformation|AttachComponentToComponent _output_get self "None" "SnapToTarget" "SnapToTarget" "KeepRelative" true)
  (Variables|Default|Setholding true)
  (UserInterface|Viewport|AddtoViewport (Variables|Default|Getindicator) 0))

(fn ConsumeInk
  (Variables|Default|Setholding false)
  (Class|IFInk|Consume(Message) (Variables|Default|GetlastHeldItem))
  (Default|AddInk (Variables|Default|Getcompanion)))

(fn GetCamCompWorld
  (return "0, 0, 0"))

(fn TryPickup
  (params (item :type Actor%20Object%20Reference))
  (if (Variables|Default|Getunlocked)
    (CallFunction|PrepforThrow item)
    (return true)
    (else
      (return false))))

(fn TryThrow
  (params (direction :type Vector :default "0, 0, 0") (strength :type Float%20%28double-precision%29))
  (Widget|RemovefromParent (Variables|Default|Getindicator))
  (if (Variables|Default|Getholding)
    (bind _outdirection (Utilities|GetThrowDirection))
    (Class|IFInk|TryThrow(Message) (Variables|Default|GetlastHeldItem) _outdirection (Variables|Default|GetthrowStrength))
    (Variables|Default|Setholding false)
    (return true)
    (else
      (return false))))