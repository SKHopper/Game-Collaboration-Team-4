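; BP_interactComp is an interaction component that lets its owner interact with whatever lies in front of a camera.
; TryInteract runs a Visibility line trace from CameraScene along its forward vector for Distance, ignoring the owner and drawing a timed debug line.
; A hit actor implementing IF_interact is stored as Interacted and receives the interface's TryInteract call, so targets define their own response.
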(fn TryInteract
  (bind _camerascene (Variables|Default|GetcameraScene))
  (bind _returnvalue (Transformation|GetWorldLocation _camerascene))
  (bind (_outhit _returnvalue_2) (Collision|LineTraceByChannel _returnvalue (+ _returnvalue (* (Math|Vector|GetForwardVector _camerascene) (Variables|Default|Getdistance))) "TraceTypeQuery1" false (Utilities|Array|MakeArray (Components|GetOwner)) "ForDuration"))
  (if _returnvalue_2
    (bind _asif_interact (Utilities|Casting|CastToIF_interact (.HitActor (Collision|BreakHitResult _outhit))))
    (bind _output_get (LocalVariables|Setinteracted _asif_interact))
    (Default|TryInteract _output_get)))