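; Music component that plays the game's background soundtrack and switches to chase music on demand.
; It spawns one persistent 2D sound, and a looping timer periodically picks a random normal track unless the player is in a chase.
; A differing pick fades out the current track, then either fades in the new one or randomly leaves silence.
; Toggling chase on fades in chase music; toggling it off fades out the audio.
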(event Custom|switchTrack
  (bind _livesound (Variables|Default|GetliveSound))
  (if (not (Variables|/Game/FirstPerson/Blueprints/BP_FirstPersonCharacter.BP_FirstPersonCharacter_C|GetinChase (Variables|Default|Getplayer)))
    (bind _output_get (Variables|Default|SetnextSound (.OutItem (Utilities|Array|Random (Variables|Default|GetnormalMusic)))))
    (if (!= _output_get (Variables|/Script/Engine.AudioComponent|GetSound (Variables|Default|GetliveSound)))
      (Audio|Components|Audio|FadeOut (Variables|Default|GetliveSound) 1.0 0.0 "Linear" :!class /Script/Engine.AudioComponent)
      (Utilities|FlowControl|Delay 1.0)
      (if (not (Math|Random|RandomBool))
        (Audio|Components|Audio|SetSound _livesound (Variables|Default|GetnextSound))
        (Audio|Components|Audio|FadeIn _livesound 1.0 0.5 0.0 "Linear" :!class /Script/Engine.AudioComponent)))))

(event Custom|toggleChase
  (params (inChase :type Boolean))
  (bind _livesound (Variables|Default|GetliveSound))
  (if inChase
    (Audio|Components|Audio|SetSound _livesound (Variables|Default|GetchaseMusic))
    (Audio|Components|Audio|FadeIn _livesound 1.0 1.0 0.0 "Linear" :!class /Script/Engine.AudioComponent)
    (else
      (Audio|Components|Audio|FadeOut _livesound 1.0 0.0 "Linear" :!class /Script/Engine.AudioComponent))))

(event EventBeginPlay
  (bind _returnvalue (Audio|SpawnSound2D "/Game/ASSET/audio/main_soundtrack/soundtrack_2_updated.soundtrack_2_updated" 0.5 1.0 0.0 0 false false))
  (Variables|Default|SetliveSound _returnvalue)
  (Utilities|Time|SetTimerbyEvent (delegate Custom|switchTrack) 3e+01 true))