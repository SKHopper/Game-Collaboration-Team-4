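; BP_friend is a companion character whose body moves along a spline to enter and exit a lantern while bobbing.
; A timeline, played forward to enter and reversed to exit, sets the body's origin on the spline and blends bob height and speed.
; Tick applies a sine-wave Z offset around that origin.
; BeginPlay also runs a delayed forward-then-reverse sequence automatically.
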(event EventBeginPlay
  (bind _bobheightinandout (Variables|Default|GetbobHeightInAndOut))
  (bind _bobspeedinandout (Variables|Default|GetbobSpeedInAndOut))
  (Utilities|FlowControl|Delay 3.0)
  (Utilities|FlowControl|Sequence
    (:then_0
      (bind _ft_linear (Timeline|TL_splineMoveBody PlayFromStart)
        (:Update
          (Variables|Default|SetbodyOriging (Utilities|FractionalSplineRelativeLocation _ft_linear))
          (Variables|Default|SetbobHeight (Math|Float|Lerp (.x _bobheightinandout) (.y _bobheightinandout) _ft_linear))
          (Variables|Default|SetbobSpeed (Math|Float|Lerp (.x _bobspeedinandout) (.y _bobspeedinandout) _ft_linear)))))
    (:then_1
      (Utilities|FlowControl|Delay 4.0)
      (Timeline|TL_splineMoveBody ReverseFromEnd))))

(event EventTick
  (params (DeltaSeconds :type Float%20%28single-precision%29))
  (CallFunction|BodyMovementTick DeltaSeconds))

(event EventExitLantern
  (bind _bobheightinandout (Variables|Default|GetbobHeightInAndOut))
  (bind _bobspeedinandout (Variables|Default|GetbobSpeedInAndOut))
  (bind _ft_linear (Timeline|TL_splineMoveBody ReverseFromEnd)
    (:Update
      (Variables|Default|SetbodyOriging (Utilities|FractionalSplineRelativeLocation _ft_linear))
      (Variables|Default|SetbobHeight (Math|Float|Lerp (.x _bobheightinandout) (.y _bobheightinandout) _ft_linear))
      (Variables|Default|SetbobSpeed (Math|Float|Lerp (.x _bobspeedinandout) (.y _bobspeedinandout) _ft_linear)))))

(event EventEntreLanter
  (bind _bobheightinandout (Variables|Default|GetbobHeightInAndOut))
  (bind _bobspeedinandout (Variables|Default|GetbobSpeedInAndOut))
  (bind _ft_linear (Timeline|TL_splineMoveBody PlayFromStart)
    (:Update
      (Variables|Default|SetbodyOriging (Utilities|FractionalSplineRelativeLocation _ft_linear))
      (Variables|Default|SetbobHeight (Math|Float|Lerp (.x _bobheightinandout) (.y _bobheightinandout) _ft_linear))
      (Variables|Default|SetbobSpeed (Math|Float|Lerp (.x _bobspeedinandout) (.y _bobspeedinandout) _ft_linear)))))

(fn ConstructionScript
  (bind _output_get (Variables|Default|SetbodyOriging (Utilities|FractionalSplineRelativeLocation 0.0)))
  (Transformation|SetRelativeLocation (Variables|Default|Getbody) _output_get false false))

(fn BodyMovementTick
  (params (frameLength :type Float%20%28double-precision%29))
  (bind _bodyoriging (Variables|Default|GetbodyOriging))
  ;[0.15 0.15 0.15 0.5] bob body on sine
  (Transformation|SetRelativeLocation (Variables|Default|Getbody) (Math|Vector|MakeVector (.x _bodyoriging) (.y _bodyoriging) (Utilities|GetBobZ)) false false))