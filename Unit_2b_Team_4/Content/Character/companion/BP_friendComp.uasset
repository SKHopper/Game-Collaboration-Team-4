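; Companion component that lets the player's friend draw markers on the floor with a limited ink supply, once the ability is activated.
; Drawing traces down from the friend and sends the hit's collision UV to actors implementing IF_friend, draining ink over time.
; Ink is clamped and mirrored to the player's HUD; toggling drives the child actor's lantern and ink effect, switching off when ink runs out.
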(event Custom|toggleDraw
  (params (on :type Boolean))
  (bind _childactor (Variables|Default|GetchildActor))
  (bind _activateddrawing (Variables|Default|GetactivatedDrawing))
  (bind _inksaved (Variables|Default|GetinkSaved))
  (bind _returnvalue (> _inksaved 0.0))
  (Default|SetInkEffect (Variables|Default|GetchildActor) (and on (and _activateddrawing _returnvalue)))
  (if _activateddrawing
    (if _returnvalue
      (if on
        (Default|EntreLanter _childactor)
        (else
          (Default|ExitLantern _childactor :!label _label)))
      (else
        (goto _label)))))

(event EventFloorDraw
  (params (hitUV :type Vector%202D%20Structure))
  ;[0.15 0.15 0.15 0.5] draw markers on floor (input from player)
  (if (stale EventActivateFloorDraw _output_get)
    (if (> (Variables|Default|GetinkSaved) 0.0)
      (bind _success (CallFunction|TryDrawDown))
      (if _success
        (CallFunction|UpdateInkSaved (* -0.5 (stale EventTick _output_get)))))))

(event EventActivateFloorDraw
  ;[0.15 0.15 0.15 0.5] draw markers on floor (input from player)
  (bind _output_get (Variables|Default|SetactivatedDrawing true))
  (CallFunction|AddInk)
  (CallFunction|AddInk)
  (CallFunction|AddInk))

(event EventBeginPlay
  (Variables|Default|Sethud (Actor|GetComponentbyClass (Game|Player|GetPlayerPawn 0) "/Game/hud/BP_hudComp.BP_hudComp_C"))
  (Utilities|FlowControl|Delay 0.2)
  (CallFunction|UpdateInkSaved -0.1))

(event EventTick
  (params (DeltaSeconds :type Float%20%28single-precision%29))
  (bind _output_get (Variables|Default|SetDelta%20Seconds DeltaSeconds)))

(fn TryDrawDown
  (bind _friendactor (Variables|Default|GetfriendActor))
  (bind _returnvalue (Transformation|GetActorLocation _friendactor))
  (bind _outhits (Class|KismetSystemLibrary|LineTraceMultiforObjects _returnvalue (- _returnvalue "0.000000,0.000000,500.000000") (Utilities|Array|MakeArray "ObjectTypeQuery2") true (Utilities|Array|MakeArray (Game|Player|GetPlayerPawn 0)) "None" true))
  (bind _array_element (Utilities|Array|ForEachLoopwithBreak _outhits)
    (:LoopBody
      (if (Utilities|DoesObjectImplementInterface (.HitActor (Collision|BreakHitResult _array_element)) "/Game/Character/companion/IF_friend.IF_friend_C")
        (Class|IFFriend|FloorDraw(Message) (.HitActor (Collision|BreakHitResult _array_element)) (.UV (Class|GameplayStatics|FindCollisionUV _array_element)))
        (return true)))
    (:Completed
      (return false))))

(fn UpdateInkSaved
  (params (delta :type Float%20%28double-precision%29))
  (bind _hud (Variables|Default|Gethud))
  (bind _hud_2 (Variables|/Game/hud/BP_hudComp.BP_hudComp_C|Gethud _hud))
  (bind _output_get (Variables|Default|SetinkSaved (Math|Float|Clamp(Float) (+ delta (Variables|Default|GetinkSaved)) 0.0 (Variables|Default|GetmaxInkSaved))))
  (Utilities|IsValid _hud
    (:Is%20Valid
      (Utilities|IsValid _hud_2
        (:Is%20Valid
          (Default|SetInk _hud_2 (/ _output_get (Variables|Default|GetmaxInkSaved))))
        (:Is%20Not%20Valid
          _)))
    (:Is%20Not%20Valid
      _))
  (if (not (> (Variables|Default|GetinkSaved) 0.0))
    (CallFunction|ToggleDraw false)))

(fn AddInk
  (CallFunction|UpdateInkSaved 1.0))