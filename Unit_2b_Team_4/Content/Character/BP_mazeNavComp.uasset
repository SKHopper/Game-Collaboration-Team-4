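; Maze navigation component that turns grid paths between two points into a world-space spline for its owner.
; On BeginPlay it gets the nav map through the maze manager interface and spawns a reusable spline actor.
; GetPathfindSpline runs Pathfind with start and target swapped, converts the cells into spline points and draws debug cones along them.
; A test event paths to a fixed location, but its looping timer is disconnected.
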(event Custom|test
  (bind _navmapcomp (Variables|Default|GetnavMapComp))
  (bind _out (Default|WorldtoNavGrid _navmapcomp (Math|Conversions|ToVector2D(Vector) (Transformation|GetActorLocation (Components|GetOwner)))))
  (bind _output_get (Variables|Default|SetmyPos _out))
  (bind _out_2 (Default|WorldtoNavGrid _navmapcomp "(X=200.000000,Y=200.000000)"))
  (CallFunction|GetPathfindSpline _output_get _out_2 1e+04))

(event EventBeginPlay
  (CallFunction|Setup))

(fn ContactMap
  (bind _outactors (Actor|GetAllActorswithInterface "/Game/ProcGen/Prototyping/IF_mazeManager.IF_mazeManager_C"))
  (bind _asif_maze_nav (Utilities|Casting|CastToIF_mazeNav (Utilities|Array|Get(acopy) (Class|Actor|GetComponentsbyInterface (Utilities|Array|Get(acopy) _outactors) "/Game/ProcGen/Prototyping/IF_mazeNav.IF_mazeNav_C"))))
  (Variables|Default|SetnavMapComp _asif_maze_nav))

(fn IsBlocked
  (params (point :type Int%20Vector%202%20Structure))
  (bind _isblocked (Default|GetIsPointBlocked (Variables|Default|GetnavMapComp) point))
  (return _isblocked))

(fn GetPathfindSpline
  (params (start :type Int%20Vector%202%20Structure) (target :type Int%20Vector%202%20Structure) (searchDistance :type Float%20%28single-precision%29))
  (bind _spline (Variables|Default|Getspline))
  (bind _spline_2 (Variables|/Game/Character/BP_mazeNavSpline.BP_mazeNavSpline_C|GetSpline _spline))
  (Spline|ClearSplinePoints (Variables|/Game/Character/BP_mazeNavSpline.BP_mazeNavSpline_C|GetSpline (Variables|Default|Getspline)) false)
  (bind _out (Default|WorldtoNavGrid (Variables|Default|GetnavMapComp) (Math|Vector2D|MakeVector2D searchDistance 0.0)))
  (bind _returnvalue (Class|MazeNavComp|Pathfind target start (Math|Conversions|ToFloat(Integer) (.x _out))))
  (if (Math|Conversions|ToBoolean(Integer) (Utilities|Array|Length _returnvalue))
    (for (_array_element _array_index) _returnvalue
      (bind _out_2 (Default|NavGridtoWorld (Variables|Default|GetnavMapComp) _array_element))
      (Spline|AddSplinePoint _spline_2 (Math|Vector|MakeVector (.x _out_2) (.y _out_2) 3.0) "World" true))
    (CallFunction|DrawSplineDebug _spline_2)
    (return true _spline_2)
    (else
      (return false 0))))

(fn Setup
  (CallFunction|ContactMap)
  (bind _returnvalue (Game|SpawnActorfromClass "/Game/Character/BP_mazeNavSpline.BP_mazeNavSpline_C" (Math|Transform|MakeTransform "0, 0, 0" "0, 0, 0" "1.000000,1.000000,1.000000") "AlwaysSpawn" "MultiplyWithRoot" 0 0))
  (Variables|Default|Setspline _returnvalue))

(fn DrawSplineDebug
  (params (InputPin :type Spline%20Component%20Object%20Reference))
  (bind _returnvalue (Class|KismetSystemLibrary|MakeLiteralInteger 70))
  (for _index (range 0 _returnvalue)
    (Class|KismetSystemLibrary|DrawDebugConeinDegrees (Spline|GetLocationatDistanceAlongSpline InputPin (* (Spline|GetSplineLength InputPin) (/ (Math|Conversions|ToFloat(Integer) _index) (Math|Conversions|ToFloat(Integer) _returnvalue))) "World") (Spline|GetDirectionatDistanceAlongSpline InputPin (* (Spline|GetSplineLength InputPin) (/ (Math|Conversions|ToFloat(Integer) _index) (Math|Conversions|ToFloat(Integer) _returnvalue))) "World") 1e+02 3e+01 3e+01 12 "(R=0.000000,G=1.000000,B=0.067034,A=1.000000)" 1.0 3.0)))