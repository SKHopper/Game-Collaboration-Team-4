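; Maze manager component that maintains a pooled population of BP_Enemy1 enemies relative to the player.
; BeginPlay pre-spawns the pool at a parking location, then a looping timer culls and activates enemies.
; Culling deactivates and parks enemies too far from the player.
; Activation randomly picks pooled enemies and teleports them to unblocked CustomNavMap cells, found by retrying candidate points, while sets track active and inactive enemies.
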(event Custom|populationUpdate
  (CallFunction|CullFarEnemies)
  (CallFunction|ActivateEnemies))

(event EventBeginPlay
  (bind _asbp_maze_manager (Utilities|Casting|CastToBP_mazeManager (Components|GetOwner)))
  (Variables|Default|SetparentManager _asbp_maze_manager)
  (Variables|Default|Setplayer (Game|Player|GetPlayerPawn 0))
  (CallFunction|PoolEnemies)
  (bind _returnvalue (Utilities|Time|SetTimerbyEvent (delegate Custom|populationUpdate) 2.0 true true -4.0))
  (Variables|Default|SetpopulationUpdateTimer _returnvalue))

(fn CullFarEnemies
  (bind _valuepin (Utilities|Set|ForEachLoop(Set) (Variables|Default|GetactivatedEnemies))
    (:then
      (bind _output_get (LocalVariables|Setenemy _valuepin))
      (if (> (Math|Vector|Distance(Vector) (Transformation|GetActorLocation _output_get) (Transformation|GetActorLocation (Variables|Default|Getplayer))) (Variables|Default|GetcullEnemyPlayerDistance))
        (Utilities|Set|Add (LocalVariables|GetculledEnemies) (LocalVariables|Getenemy))
        (Utilities|Set|Add (Variables|Default|GetdeactivatedEnemies) (LocalVariables|Getenemy))
        (Transformation|SetActorLocation (LocalVariables|Getenemy) "0.000000,0.000000,1000.000000" false true)))
    (:CompletedPin
      (bind _result (Utilities|Set|ToArray (LocalVariables|GetculledEnemies)))
      (Utilities|Set|RemoveItems (Variables|Default|GetactivatedEnemies) _result)
      (for _array_element _result
        (Default|Deactivate _array_element)))))

(fn ActivateEnemies
  (if (Math|Conversions|ToBoolean(Integer) (Utilities|Set|Length (Variables|Default|GetdeactivatedEnemies)))
    (bind _valuepin (Utilities|Set|ForEachLoop(Set) (Variables|Default|GetdeactivatedEnemies))
      (:then
        (if (Math|Random|RandomBoolwithWeight (Variables|Default|GetchanceSpawnEnemy))
          (Utilities|Set|Add (Variables|Default|GetactivatedEnemies) _valuepin)
          (Utilities|Set|Add (LocalVariables|GetunculledEnemies) _valuepin)
          (bind _returnvalue (CallFunction|GetEnemySpawnGridPoint))
          (Transformation|SetActorLocation _valuepin _returnvalue false true)
          (else
            (bind _result (Utilities|Set|ToArray (LocalVariables|GetunculledEnemies) :!label _label))
            (Utilities|Set|RemoveItems (Variables|Default|GetdeactivatedEnemies) _result)
            (for _array_element _result
              (Default|Activate _array_element)))))
      (:CompletedPin
        (goto _label)))))

(fn PoolEnemies
  (for _index (range 0 (- (Variables|Default|GetmaxPopulation) 1))
    (bind _returnvalue (Game|SpawnActorfromClass "/Game/Character/Enemies/BP_Enemy1.BP_Enemy1_C" (Math|Transform|MakeTransform "0.000000,0.000000,1000.000000" "0, 0, 0" "1.000000,1.000000,1.000000") "AdjustIfPossibleButAlwaysSpawn" "MultiplyWithRoot" 0 0))
    (Utilities|Set|Add (Variables|Default|GetdeactivatedEnemies) _returnvalue)))

(fn GetEnemySpawnGridPoint
  (bind _parentmanager (Variables|Default|GetparentManager))
  (bind _customnavmap (Variables|/Game/ProcGen/Prototyping/BP_mazeManager.BP_mazeManager_C|GetcustomNavMap _parentmanager))
  (Utilities|FlowControl|ForLoopwithBreak 0 999 :!label _label
    (:LoopBody
      (bind _out (Default|WorldtoNavGrid _customnavmap (Math|Conversions|ToVector2D(Vector) (Utilities|GetRandomEnemySpawn))))
      (bind _isblocked (Default|GetIsPointBlocked _customnavmap _out))
      (if (not _isblocked)
        (bind _out_2 (Default|NavGridtoWorld _customnavmap _out))
        (LocalVariables|SetoutPoint _out_2)
        (goto _label Break)))
    (:Completed
      (return (Math|Conversions|ToVector(Vector2D) (LocalVariables|GetoutPoint) 2e+02)))))